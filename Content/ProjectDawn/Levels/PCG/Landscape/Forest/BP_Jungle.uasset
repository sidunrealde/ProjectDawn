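; BP_Jungle is a jungle Blueprint in the PCG landscape forest set that exposes on/off toggles for scatter categories.
; Its construction script turns each toggle for trees, bushes, shrubs, grass, detail plants, shore foliage, rocks and path into a full or zero density variable.
; The path toggle drives pebble density.
; The event graph has no logic, and nothing here shows what consumes the densities.
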(event EventBeginPlay)

(event Collision|EventActorBeginOverlap
  (params (OtherActor :type Actor%20Object%20Reference)))

(event EventTick
  (params (DeltaSeconds :type Float%20%28single-precision%29)))

(fn ConstructionScript
  (Variables|Default|SetDetailPlantDensity (select (Variables|Config|Detail|GetbEnableDetailPlants) 1.0 0.0))
  (Variables|Default|SetShrubDensity (select (Variables|Config|Detail|GetbEnableShrubs) 1.0 0.0))
  (Variables|Default|SetGrassDensity (select (Variables|Config|Detail|GetbEnableGrass) 1.0 0.0))
  (Variables|Default|SetPebbleDensity (select (Variables|Config|Main|GetbEnablePath) 1.0 0.0))
  (Variables|Default|SetTreeDensity (select (Variables|Config|Main|GetbEnableTrees) 1.0 0.0))
  (Variables|Default|SetShoreShrubsDensity (select (Variables|Config|Detail|GetbEnableShoreFoliage) 1.0 0.0))
  (Variables|Default|SetRockDensity (select (Variables|Config|Main|GetbEnableRocks) 1.0 0.0))
  (Variables|Default|SetBushDensity (select (Variables|Config|Detail|GetbEnableBushes) 1.0 0.0)))