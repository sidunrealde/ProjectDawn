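; Base projectile actor for spells, configured at construction from its DT_Spells row, which sets speed and gravity.
; On spawn it plays a sound and destroys itself after a fixed lifetime.
; On overlap, Ranged spells send hit, elemental effect and effect-duration messages to Enemy-tagged actors, then end.
; Trap spells fire ExplodeOnHit once on any overlap and self-destruct; that event and the ImpactRadius overlap are empty here.
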(event OnComponentBeginOverlap(ImpactRadius)
  (params (OverlappedComponent :type Primitive%20Component%20Object%20Reference) (OtherActor :type Actor%20Object%20Reference) (OtherComp :type Primitive%20Component%20Object%20Reference) (OtherBodyIndex :type Integer) (bFromSweep :type Boolean) (SweepResult :type Hit%20Result%20Structure%20%28by%20ref%29)))

(event Custom|ExplodeOnHit)

(event EventBeginPlay
  (bind _returnvalue (Audio|SpawnSoundatLocation (Variables|Default|GetAudioTrack) (Transformation|GetActorLocation) "0, 0, 0" 1.0 1.0 0.0 0 0))
  (Variables|Default|SetSoundEffect _returnvalue)
  (Utilities|FlowControl|Delay 6.0)
  (Audio|Components|Audio|Stop (Variables|Default|GetSoundEffect))
  (Actor|DestroyActor))

(event Collision|EventActorBeginOverlap
  (params (OtherActor :type Actor%20Object%20Reference))
  (bind _spellinfo (Variables|Default|GetSpellInfo))
  (bind (_spelltype _elementaltype _potency _duration) (Utilities|Struct|BreakDS_SpellInfo _spellinfo))
  (switch Utilities|FlowControl|Switch|SwitchonEN_SpellType (Utilities|Struct|BreakDS_SpellInfo (Variables|Default|GetSpellInfo))
    (:NewEnumerator0
      (if (Actor|ActorHasTag OtherActor "Enemy")
        (Class|BPIArrowHit|OnEnemyArrowHit(Message) OtherActor)
        (Class|BPIStatusEffect|ElementalEffect(Message) OtherActor _potency _spelltype _elementaltype)
        (Class|BPIStatusEffect|TimerEndEffect(Message) OtherActor _duration _elementaltype)
        (Audio|Components|Audio|Stop (Variables|Default|GetSoundEffect))
        (Actor|DestroyActor)))
    (:NewEnumerator2
      (if true
        (Utilities|FlowControl|DoOnce false
          (:Completed
            (CallFunction|ExplodeonHit)
            (Actor|DestroyActor)))))))

(fn ConstructionScript
  (bind _projectilemovement (Variables|Default|GetProjectileMovement))
  (bind _returnvalue (Utilities|GetDataTableRow "/Game/ProjectDawn/Blueprints/Magic/Data/DT_Spells.DT_Spells" (Utilities|String|StringToName (Utilities|String|EnumtoString (.SpellName (Utilities|Struct|BreakDS_SpellInfo (Variables|Default|GetSpellInfo))))))
    (:then
      (bind _output_get (Variables|Default|SetSpellInfo _returnvalue))
      (Variables|/Script/Engine.ProjectileMovementComponent|SetInitialSpeed _projectilemovement (.Speed (Utilities|Struct|BreakDS_SpellInfo _output_get)))
      (Variables|/Script/Engine.ProjectileMovementComponent|SetMaxSpeed _projectilemovement (.Speed (Utilities|Struct|BreakDS_SpellInfo _output_get)))
      (Variables|/Script/Engine.ProjectileMovementComponent|SetProjectileGravityScale _projectilemovement (.GravityScale (Utilities|Struct|BreakDS_SpellInfo _output_get))))))