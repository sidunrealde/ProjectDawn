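; Thunder trap actor in the magic trap set that turns into its spawned trap effect when it explodes on hit.
; Its ExplodeonHit event spawns BPC_ThunderTrapSpawn at the actor's transform, stops its sound effect and destroys the actor.
; The construction script defers to the parent class, and the overlap and tick events are disabled stubs.
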(event Collision|EventActorBeginOverlap
  (params (OtherActor :type Actor%20Object%20Reference))
  (|CallParentFunction OtherActor) ; This node is disabled and will not be called.\nDrag off pins to build functionality.
)

(event EventTick
  (params (DeltaSeconds :type Float%20%28single-precision%29))
  (|CallParentFunction DeltaSeconds) ; This node is disabled and will not be called.\nDrag off pins to build functionality.
)

(event EventExplodeonHit
  (Game|SpawnActorfromClass "/Game/ProjectDawn/Blueprints/Magic/Traps/BPC_ThunderTrapSpawn.BPC_ThunderTrapSpawn_C" (Transformation|GetActorTransform) "Undefined" "OverrideRootScale" 0 0)
  (Audio|Components|Audio|Stop (Variables|Default|GetSoundEffect))
  (Actor|DestroyActor))

(fn ConstructionScript
  (|CallParentFunction))