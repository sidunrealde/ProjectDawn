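; BPC_ShieldWall is a defensive buff spell actor that shields the player's hero for a limited time.
; On BeginPlay it attaches to the BP_HeroBase player character's mesh and calls Defense with the potency and duration from SpellInfo.
; A 2D shield sound plays until that duration elapses, then the actor destroys itself.
; The particle-finished destroy handler is never bound, so the delay alone drives cleanup.
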(event Custom|OnSystemFinished_Event
  (params (PSystem :type Particle%20System%20Component%20Object%20Reference))
  (Actor|DestroyActor))

(event EventBeginPlay
  (bind _spellinfo (Variables|Default|GetSpellInfo))
  (bind (_elementaltype _potency _duration) (Utilities|Struct|BreakDS_SpellInfo _spellinfo))
  (|CallParentFunction)
  (bind _asbp_hero_base (Utilities|Casting|CastToBP_HeroBase (Game|GetPlayerCharacter 0)))
  (Transformation|AttachComponentToComponent (Variables|/Script/Engine.Character|GetMesh _asbp_hero_base) "None" "SnapToTarget" "SnapToTarget" "SnapToTarget" true)
  (Default|Defense+ _asbp_hero_base _potency _duration)
  (bind _returnvalue (Audio|SpawnSound2D "/Game/ProjectDawn/Blueprints/Sounds/Magic/Magic_Shield_Cue.Magic_Shield_Cue" 1.0 1.0 0.0 0))
  (Utilities|FlowControl|Delay _duration)
  (Audio|Components|Audio|Stop _returnvalue)
  (Actor|DestroyActor))

(event Collision|EventActorBeginOverlap
  (params (OtherActor :type Actor%20Object%20Reference))
  (|CallParentFunction OtherActor) ; This node is disabled and will not be called.\nDrag off pins to build functionality.
)

(event EventTick
  (params (DeltaSeconds :type Float%20%28single-precision%29))
  (|CallParentFunction DeltaSeconds) ; This node is disabled and will not be called.\nDrag off pins to build functionality.
)

(fn ConstructionScript
  (|CallParentFunction))