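; BP_TrapBase is a magic trap spell actor that applies elemental effects to overlapping Enemy-tagged actors.
; The construction script loads SpellInfo from DT_Spells using the spell name.
; On BeginPlay it plays a sound and traces downward; only on a hit does it snap to ground, then destroy itself after the spell's duration.
; Sphere overlaps message enemies to register a hit and manage timed effects, shortening the timer on exit.
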(event OnComponentBeginOverlap(Sphere)
  (params (OverlappedComponent :type Primitive%20Component%20Object%20Reference) (OtherActor :type Actor%20Object%20Reference) (OtherComp :type Primitive%20Component%20Object%20Reference) (OtherBodyIndex :type Integer) (bFromSweep :type Boolean) (SweepResult :type Hit%20Result%20Structure%20%28by%20ref%29))
  (bind _spellinfo (Variables|Default|GetSpellInfo))
  (bind (_spelltype _elementaltype _potency _duration) (Utilities|Struct|BreakDS_SpellInfo _spellinfo))
  (if (Actor|ActorHasTag OtherActor "Enemy")
    (Class|BPIArrowHit|OnEnemyArrowHit(Message) OtherActor)
    (switch Utilities|FlowControl|Switch|SwitchonEN_SpellType _spelltype
      (:NewEnumerator2
        (Class|BPIStatusEffect|ElementalEffect(Message) OtherActor _potency _spelltype _elementaltype)
        (Class|BPIStatusEffect|TimerEndEffect(Message) OtherActor _duration _elementaltype)))))

(event OnComponentEndOverlap(Sphere)
  (params (OverlappedComponent :type Primitive%20Component%20Object%20Reference) (OtherActor :type Actor%20Object%20Reference) (OtherComp :type Primitive%20Component%20Object%20Reference) (OtherBodyIndex :type Integer))
  (if (Actor|ActorHasTag OtherActor "Enemy")
    (Class|BPIStatusEffect|TimerEndEffect(Message) OtherActor 0.2 (.ElementalType (Utilities|Struct|BreakDS_SpellInfo (Variables|Default|GetSpellInfo))))))

(event EventBeginPlay
  (bind _returnvalue (Transformation|GetActorLocation))
  (Utilities|FlowControl|Sequence
    (:then_0
      (bind _returnvalue_2 (Audio|SpawnSoundatLocation (Variables|Default|GetAudioTrack) (Transformation|GetActorLocation) "0, 0, 0" 1.0 1.0 0.0 0 0))
      (Variables|Default|SetSound _returnvalue_2)
      (bind (_outhit _returnvalue_3) (Collision|LineTraceByChannel _returnvalue (- _returnvalue "0.000000,0.000000,300.000000") "TraceTypeQuery1" false 0 "None"))
      (if _returnvalue_3
        (Transformation|SetActorLocation (.Location (Collision|BreakHitResult _outhit)) false false)
        (Utilities|FlowControl|Delay (Utilities|Struct|BreakDS_SpellInfo (Variables|Default|GetSpellInfo)))
        (Audio|Components|Audio|Stop (Variables|Default|GetSound))
        (Actor|DestroyActor)))))

(fn ConstructionScript
  (bind _returnvalue (Utilities|GetDataTableRow "/Game/ProjectDawn/Blueprints/Magic/Data/DT_Spells.DT_Spells" (Utilities|String|StringToName (Utilities|String|EnumtoString (.SpellName (Utilities|Struct|BreakDS_SpellInfo (Variables|Default|GetSpellInfo))))))
    (:then
      (Variables|Default|SetSpellInfo _returnvalue))))