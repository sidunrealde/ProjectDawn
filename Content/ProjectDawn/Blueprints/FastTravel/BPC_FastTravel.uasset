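; Fast travel point that the player unlocks by walking into its sphere and uses through a fast travel menu.
; First overlap registers it in the hero's ActivatedFastTravelPoints and lights the fire effect, which ReLight can also trigger.
; Interact toggles a cached W_FastTravel widget unless another hero screen is open, switching input mode, cursor and the player controller's CustomTimeDilation.
; Leaving the sphere closes the menu.
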(event OnComponentBeginOverlap(Sphere)
  (params (OverlappedComponent :type Primitive%20Component%20Object%20Reference) (OtherActor :type Actor%20Object%20Reference) (OtherComp :type Primitive%20Component%20Object%20Reference) (OtherBodyIndex :type Integer) (bFromSweep :type Boolean) (SweepResult :type Hit%20Result%20Structure%20%28by%20ref%29))
  (bind _self self)
  (bind _playerref (Variables|Default|GetPlayerRef))
  (bind _activatedfasttravelpoints (Variables|/Game/ProjectDawn/Blueprints/BP_HeroBase.BP_HeroBase_C|GetActivatedFastTravelPoints _playerref))
  (if (Actor|ActorHasTag OtherActor "Player")
    (if (not (Utilities|Array|ContainsItem _activatedfasttravelpoints _self))
      (Utilities|Array|AddUnique _activatedfasttravelpoints _self)
      (Components|Activation|Activate (Variables|Default|Getfire) true))))

(event OnComponentEndOverlap(Sphere)
  (params (OverlappedComponent :type Primitive%20Component%20Object%20Reference) (OtherActor :type Actor%20Object%20Reference) (OtherComp :type Primitive%20Component%20Object%20Reference) (OtherBodyIndex :type Integer))
  (if (and (Variables|Default|GetIsMenuOpen) (Actor|ActorHasTag OtherActor "Player"))
    (CallFunction|CheckifMenuNeedstoClose)))

(event Custom|ReLight
  (Components|Activation|Activate (Variables|Default|Getfire) true))

(event Custom|CheckIfMenuNeedsToClose
  (bind _returnvalue (Game|GetPlayerController 0))
  (bind _returnvalue_2 (Game|GetPlayerController 0))
  (if (Variables|Default|GetIsMenuOpen)
    (Widget|RemovefromParent (Variables|Default|GetFastTravelWidgetRef))
    (Input|SetInputModeGameOnly _returnvalue false)
    (Variables|/Script/Engine.PlayerController|SetbShowMouseCursor _returnvalue false)
    (Variables|/Script/Engine.Actor|SetCustomTimeDilation _returnvalue 1.0)
    (Variables|Default|SetIsMenuOpen false)
    (else
      (Utilities|IsValid (Variables|Default|GetFastTravelWidgetRef)
        (:Is%20Valid
          _)
        (:Is%20Not%20Valid
          (bind _returnvalue_3 (UserInterface|CreateWidget "/Game/ProjectDawn/Blueprints/HUD/FastTravel/W_FastTravel.W_FastTravel_C"))
          (bind _output_get (Variables|Default|SetFastTravelWidgetRef _returnvalue_3))))
      (UserInterface|Viewport|AddtoViewport _output_get 0)
      (Variables|Default|SetIsMenuOpen true)
      (Input|SetInputModeGameandUI _returnvalue_2 _output_get "DoNotLock" true false)
      (Variables|/Script/Engine.PlayerController|SetbShowMouseCursor _returnvalue_2 true)
      (Variables|/Script/Engine.Actor|SetCustomTimeDilation _returnvalue_2 0.001))))

(event EventBeginPlay
  (bind _asbp_hero_base (Utilities|Casting|CastToBP_HeroBase (Game|GetPlayerCharacter 0)))
  (Variables|Default|SetPlayerRef _asbp_hero_base))

(event EventInteract
  (bind _returnvalue (Game|GetPlayerController 0))
  (bind _returnvalue_2 (Game|GetPlayerController 0))
  (bind _playerref (Variables|Default|GetPlayerRef))
  (if (not (Math|Boolean|ORBoolean (Variables|/Game/ProjectDawn/Blueprints/BP_HeroBase.BP_HeroBase_C|GetIsCraftingScreenOpen _playerref) (Variables|/Game/ProjectDawn/Blueprints/BP_HeroBase.BP_HeroBase_C|GetIsEnemyLootScreenOpen _playerref) (Variables|/Game/ProjectDawn/Blueprints/BP_HeroBase.BP_HeroBase_C|GetIsMenuOpen _playerref) (Variables|/Game/ProjectDawn/Blueprints/BP_HeroBase.BP_HeroBase_C|GetIsQuestLogOpen _playerref) (Variables|/Game/ProjectDawn/Blueprints/BP_HeroBase.BP_HeroBase_C|GetIsSpellBookOpen _playerref) (Variables|/Game/ProjectDawn/Blueprints/BP_HeroBase.BP_HeroBase_C|GetIsSaveScreenOpen _playerref)))
    (if (Variables|Default|GetIsMenuOpen)
      (Widget|RemovefromParent (Variables|Default|GetFastTravelWidgetRef))
      (Input|SetInputModeGameOnly _returnvalue false)
      (Variables|/Script/Engine.PlayerController|SetbShowMouseCursor _returnvalue false)
      (Variables|/Script/Engine.Actor|SetCustomTimeDilation _returnvalue 1.0)
      (Variables|Default|SetIsMenuOpen false)
      (else
        (Utilities|IsValid (Variables|Default|GetFastTravelWidgetRef)
          (:Is%20Valid
            _)
          (:Is%20Not%20Valid
            (bind _returnvalue_3 (UserInterface|CreateWidget "/Game/ProjectDawn/Blueprints/HUD/FastTravel/W_FastTravel.W_FastTravel_C"))
            (bind _output_get (Variables|Default|SetFastTravelWidgetRef _returnvalue_3))))
        (UserInterface|Viewport|AddtoViewport _output_get 0)
        (Variables|Default|SetIsMenuOpen true)
        (Input|SetInputModeGameandUI _returnvalue_2 _output_get "DoNotLock" true false)
        (Variables|/Script/Engine.PlayerController|SetbShowMouseCursor _returnvalue_2 true)
        (Variables|/Script/Engine.Actor|SetCustomTimeDilation _returnvalue_2 0.001)))))

(fn ConstructionScript
  (|CallParentFunction))