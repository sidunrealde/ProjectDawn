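; Loot box logic that lets the player loot dead enemies and chests through a HUD list.
; LootMenu fills LootTable with W_LootIcon widgets from DT_ItemInfo and switches to UI input, or closes the list if already populated.
; SelectRandomLoot rolls each LootPool item into LootDrop with a random quantity, repeating on later opens until something drops.
; ClearLootWidget restores game input and marks the box looted once LootDrop is empty.
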(event Custom|LootMenu
  (bind _returnvalue (Game|GetPlayerController 0))
  (bind _returnvalue_2 (Game|GetPlayerController 0))
  (bind _lootdrop (Variables|Default|GetLootDrop))
  (if (or (Variables|Default|GetIsDead) (Variables|Default|GetIsChest))
    (if (not (Variables|Default|GetIsLooted))
      (if (Variables|Default|GetIsRandomLootAssigned)
        _
        (else
          (CallFunction|SelectRandomLoot)))
      (if (Utilities|Map|IsNotEmpty (Variables|Default|GetLootDrop))
        (bind _asbp_hero_base (Utilities|Casting|CastToBP_HeroBase (Game|GetPlayerCharacter 0)))
        (bind _output_get (Variables|Default|SetPlayerRef _asbp_hero_base))
        (if (Class|PanelWidget|HasAnyChildren (Variables|/Game/ProjectDawn/Blueprints/HUD/W_PlayerHUD.W_PlayerHUD_C|GetLootTable (Variables|/Game/ProjectDawn/Blueprints/BP_HeroBase.BP_HeroBase_C|GetHUDRef _output_get)))
          (Widget|Panel|ClearChildren (Variables|/Game/ProjectDawn/Blueprints/HUD/W_PlayerHUD.W_PlayerHUD_C|GetLootTable (Variables|/Game/ProjectDawn/Blueprints/BP_HeroBase.BP_HeroBase_C|GetHUDRef _output_get)))
          (Input|SetInputModeGameOnly _returnvalue_2 false)
          (Variables|/Script/Engine.PlayerController|SetbShowMouseCursor _returnvalue_2 false)
          (Variables|Default|SetIsLootScreenOpen false)
          (Variables|/Game/ProjectDawn/Blueprints/BP_HeroBase.BP_HeroBase_C|SetIsEnemyLootScreenOpen (Variables|Default|GetPlayerRef) false)
          (else
            (Variables|/Game/ProjectDawn/Blueprints/HUD/W_PlayerHUD.W_PlayerHUD_C|SetLootRef (Variables|/Game/ProjectDawn/Blueprints/BP_HeroBase.BP_HeroBase_C|GetHUDRef _output_get) self)
            (bind _keys (Utilities|Map|Keys _lootdrop))
            (bind _values (Utilities|Map|Values _lootdrop))
            (for (_array_element _array_index) _keys
              (bind _returnvalue_3 (Utilities|GetDataTableRow "/Game/ProjectDawn/Blueprints/Items/Data/DT_ItemInfo.DT_ItemInfo" (Utilities|String|StringToName (Utilities|String|EnumtoString _array_element)))
                (:then
                  (bind _returnvalue_4 (UserInterface|CreateWidget "/Game/ProjectDawn/Blueprints/HUD/W_LootIcon.W_LootIcon_C" 0 _returnvalue_3 self (Utilities|Array|Get(acopy) _values _array_index)))
                  (Class|VerticalBox|AddChildtoVerticalBox (Variables|/Game/ProjectDawn/Blueprints/HUD/W_PlayerHUD.W_PlayerHUD_C|GetLootTable (Variables|/Game/ProjectDawn/Blueprints/BP_HeroBase.BP_HeroBase_C|GetHUDRef (Variables|Default|GetPlayerRef))) _returnvalue_4))))
            (Input|SetInputModeGameandUI _returnvalue _returnvalue_4 "DoNotLock" true false)
            (Variables|/Script/Engine.PlayerController|SetbShowMouseCursor _returnvalue true)
            (Variables|/Game/ProjectDawn/Blueprints/BP_HeroBase.BP_HeroBase_C|SetIsEnemyLootScreenOpen (Variables|Default|GetPlayerRef) true)
            (Variables|Default|SetIsLootScreenOpen true)))))))

(event Custom|ClearLootWidget
  (bind _returnvalue (Game|GetPlayerController 0))
  (if (Variables|Default|GetIsLootScreenOpen)
    (if (Utilities|Map|IsEmpty (Variables|Default|GetLootDrop))
      (Variables|Default|SetIsLooted true))
    (Widget|Panel|ClearChildren (Variables|/Game/ProjectDawn/Blueprints/HUD/W_PlayerHUD.W_PlayerHUD_C|GetLootTable (Variables|/Game/ProjectDawn/Blueprints/BP_HeroBase.BP_HeroBase_C|GetHUDRef (stale Custom|LootMenu _output_get))))
    (Input|SetInputModeGameOnly _returnvalue false)
    (Variables|/Script/Engine.PlayerController|SetbShowMouseCursor _returnvalue false)
    (Variables|Default|SetIsLootScreenOpen false)
    (Variables|/Game/ProjectDawn/Blueprints/BP_HeroBase.BP_HeroBase_C|SetIsEnemyLootScreenOpen (Variables|Default|GetPlayerRef) false)))

(fn SelectRandomLoot
  (bind _lootpool (Variables|Default|GetLootPool))
  (bind _keys (Utilities|Map|Keys _lootpool))
  (bind _values (Utilities|Map|Values _lootpool))
  (for (_array_element _array_index) _keys
    (if (Math|Random|RandomBoolwithWeight (Variables|Default|GetLootDropChance))
      (Utilities|Map|Add (Variables|Default|GetLootDrop) _array_element (Math|Random|RandomIntegerinRange 1 (Utilities|Array|Get(acopy) _values _array_index)))
      (Variables|Default|SetIsRandomLootAssigned true))))

(fn QuestInteract
  (return ""))