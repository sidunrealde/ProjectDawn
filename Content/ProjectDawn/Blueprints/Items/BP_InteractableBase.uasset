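; BP_InteractableBase is the base actor for world items the player can interact with, showing item info and picking them up.
; The construction script loads ItemInfo from DT_ItemInfo using the ItemName enum as row name.
; Sphere overlaps toggle the info message on the overlapping actor.
; Interact sends a pickup message to the player, plays a sound and optionally destroys the item; QuestInteract exposes an objective ID.
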(event OnComponentBeginOverlap(Sphere)
  (params (OverlappedComponent :type Primitive%20Component%20Object%20Reference) (OtherActor :type Actor%20Object%20Reference) (OtherComp :type Primitive%20Component%20Object%20Reference) (OtherBodyIndex :type Integer) (bFromSweep :type Boolean) (SweepResult :type Hit%20Result%20Structure%20%28by%20ref%29))
  (if (Variables|Default|GetInteractable)
    (Class|BPIInteract|DisplayInfo(Message) OtherActor (Variables|Default|GetItemInfo) true)))

(event OnComponentEndOverlap(Sphere)
  (params (OverlappedComponent :type Primitive%20Component%20Object%20Reference) (OtherActor :type Actor%20Object%20Reference) (OtherComp :type Primitive%20Component%20Object%20Reference) (OtherBodyIndex :type Integer))
  (Class|BPIInteract|DisplayInfo(Message) :self OtherActor))

(event EventInteract
  (if (Variables|Default|GetInteractable)
    (Class|BPIInteract|PickUp(Message) (Game|GetPlayerCharacter 0) (Variables|Default|GetItemInfo))
    (if (Variables|Default|GetShouldDestroy)
      (Audio|PlaySound2D "/Game/Interface_And_Item_Sounds/Cues/Abstract_Pop_05_Cue.Abstract_Pop_05_Cue" 1.0 1.0 0.0 0 0)
      (Actor|DestroyActor)
      (else
        (Audio|PlaySound2D "/Game/Interface_And_Item_Sounds/Cues/Musical_Click_08_Cue.Musical_Click_08_Cue" 1.0 1.0 0.0 0 0)))))

(fn ConstructionScript
  (bind _returnvalue (Utilities|GetDataTableRow "/Game/ProjectDawn/Blueprints/Items/Data/DT_ItemInfo.DT_ItemInfo" (Utilities|String|StringToName (Utilities|String|EnumtoString (Variables|Default|GetItemName))))
    (:then
      (Variables|Default|SetItemInfo _returnvalue))))

(fn ElementalCheck
  (params (ElementType :type EN_ElementalTypes%20Enum :default "NewEnumerator0"))
  (Variables|Default|SetElementalType ElementType))

(fn QuestInteract
  (return (Variables|Default|GetObjective%20ID)))