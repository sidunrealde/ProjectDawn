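; Lootable chest Blueprint that opens a loot menu when interacted with, using an inherited or attached BCLootBox component named from ChestName at BeginPlay.
; Interact calls the loot menu every time, while a DoOnce plays the lid and base opening animations only the first time.
; A sphere overlap by a Player-tagged actor clears Interactable once the loot box reports it is looted.
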(event OnComponentBeginOverlap(Sphere)
  (params (OverlappedComponent :type Primitive%20Component%20Object%20Reference) (OtherActor :type Actor%20Object%20Reference) (OtherComp :type Primitive%20Component%20Object%20Reference) (OtherBodyIndex :type Integer) (bFromSweep :type Boolean) (SweepResult :type Hit%20Result%20Structure%20%28by%20ref%29))
  (if (and (Variables|/Game/ProjectDawn/Blueprints/Items/BC_LootBox.BC_LootBox_C|GetIsLooted (Variables|Default|GetBC_LootBox)) (Actor|ActorHasTag OtherActor "Player"))
    (Variables|Default|SetInteractable false)))

(event EventBeginPlay
  (Variables|/Game/ProjectDawn/Blueprints/Items/BC_LootBox.BC_LootBox_C|SetLootName (Variables|Default|GetBC_LootBox) (Variables|Default|GetChestName)))

(event EventInteract
  (Default|LootMenu (Variables|Default|GetBC_LootBox))
  (Utilities|FlowControl|DoOnce false
    (:Completed
      (Components|Animation|PlayAnimation (Variables|Default|GetChestLid) "/Game/ProjectDawn/Props/Chest/chest_anim_top_Open.chest_anim_top_Open" false)
      (Components|Animation|PlayAnimation (Variables|Default|GetChestBase) "/Game/ProjectDawn/Props/Chest/chest_anim_bot_Anim.chest_anim_bot_Anim" false))))

(fn ConstructionScript
  (|CallParentFunction))