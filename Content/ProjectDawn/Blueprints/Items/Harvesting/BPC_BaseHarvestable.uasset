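; Base Blueprint for harvestable world objects that break after repeated hits and drop items.
; Each damage event removes one Health regardless of damage amount.
; At zero Health it spawns a random count of the configured class, bounded by min and max harvest values, scattered slightly above the Item component, then destroys itself.
; A cast to BP_HeroBase is present but never runs.
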(event Game|Damage|EventAnyDamage
  (params (Damage :type Float%20%28single-precision%29) (DamageType :type Damage%20Type%20Object%20Reference) (InstigatedBy :type Controller%20Object%20Reference) (DamageCauser :type Actor%20Object%20Reference))
  (bind _result (Math|Integer|DecrementInt (Variables|Default|GetHealth))
    (:%20%20
      (if (<= _result 0)
        (for _index (range 0 (Math|Random|RandomIntegerinRange (Variables|Default|GetMinItemsToHarvest) (Variables|Default|GetMaxItemsToHarvest)))
          (Game|SpawnActorfromClass (Variables|Default|GetClass) (Math|Transform|MakeTransform (+ (Transformation|GetWorldLocation (Variables|Default|GetItem)) (Math|Vector|MakeVector (Math|Random|RandomFloatinRange -5.0 5.0) (Math|Random|RandomFloatinRange -5.0 5.0) 5e+01)) "0, 0, 0" "1.000000,1.000000,1.000000") "Undefined" "SelectDefaultAtRuntime" 0 0))
        (Actor|DestroyActor)))))

(fn ConstructionScript
  (|CallParentFunction))