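; Wood arrow projectile that takes its base damage from the player hero's bow potency on spawn.
; Box overlap with an Enemy-tagged actor sends a hit message, applies damage and destroys the arrow.
; Fire, Freeze and Shock arrows also send elemental effect and timed end-effect messages.
; ElementalCheck extends the parent with attached emitters but switches on fixed Physical, so none spawn; drop and release-noise logic is unwired.
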(event OnComponentBeginOverlap(Box)
  (params (OverlappedComponent :type Primitive%20Component%20Object%20Reference) (OtherActor :type Actor%20Object%20Reference) (OtherComp :type Primitive%20Component%20Object%20Reference) (OtherBodyIndex :type Integer) (bFromSweep :type Boolean) (SweepResult :type Hit%20Result%20Structure%20%28by%20ref%29))
  (bind _elementaltype (Variables|Default|GetElementalType))
  (Utilities|IsValid OtherActor
    (:Is%20Valid
      (if (Actor|ActorHasTag OtherActor "Enemy")
        (Variables|Default|SetHit%20Component 0)
        (Class|BPIArrowHit|OnEnemyArrowHit(Message) OtherActor)
        (switch Utilities|FlowControl|Switch|SwitchonEN_ElementalTypes _elementaltype
          (:NewEnumerator0
            _)
          (:NewEnumerator1
            (Class|BPIStatusEffect|ElementalEffect(Message) OtherActor 2.0 "NewEnumerator0" _elementaltype :!label _label)
            (Class|BPIStatusEffect|TimerEndEffect(Message) OtherActor 3.0 _elementaltype))
          (:NewEnumerator2
            (goto _label))
          (:NewEnumerator3
            (goto _label)))
        (Game|Damage|ApplyDamage OtherActor (Variables|Default|GetBase%20Damage) 0 (Game|GetPlayerCharacter 0))
        (Actor|DestroyActor)))))

(event OnComponentHit(Item)
  (params (HitComponent :type Primitive%20Component%20Object%20Reference) (OtherActor :type Actor%20Object%20Reference) (OtherComp :type Primitive%20Component%20Object%20Reference) (NormalImpulse :type Vector :default "0, 0, 0") (Hit :type Hit%20Result%20Structure%20%28by%20ref%29)))

(event EventBeginPlay
  (bind _asbp_hero_base (Utilities|Casting|CastToBP_HeroBase (Game|GetPlayerCharacter 0)))
  (Variables|Default|SetBase%20Damage (Utilities|Struct|BreakDS_ItemInfo (Variables|/Game/ProjectDawn/Blueprints/BP_HeroBase.BP_HeroBase_C|GetBowInfo _asbp_hero_base))))

(fn ConstructionScript
  (|CallParentFunction))

(fn ElementalCheck
  (params (ElementType :type EN_ElementalTypes%20Enum :default "NewEnumerator0"))
  (|CallParentFunction ElementType)
  (switch Utilities|FlowControl|Switch|SwitchonEN_ElementalTypes "NewEnumerator0"
    (:NewEnumerator1
      (Effects|SpawnEmitterAttached "/Game/ProjectDawn/FX/CascadeParticleSystem/Spells/Ranged/Fireball/P_FireBall_Base.P_FireBall_Base" (Variables|Default|GetItem) "None" "0, 0, 0" "0, 0, 0" "1.000000,1.000000,1.000000" "SnapToTargetIncludingScale"))
    (:NewEnumerator2
      (Effects|SpawnEmitterAttached "/Game/FXVarietyPack/Particles/P_ky_waterBall.P_ky_waterBall" (Variables|Default|GetItem) "None" "0, 0, 0" "0, 0, 0" "1.000000,1.000000,1.000000" "SnapToTargetIncludingScale"))
    (:NewEnumerator3
      (Effects|SpawnEmitterAttached "/Game/FXVarietyPack/Particles/P_ky_shootingStar1.P_ky_shootingStar1" (Variables|Default|GetItem) "None"))))

(fn EnemyRef
  (return 0))