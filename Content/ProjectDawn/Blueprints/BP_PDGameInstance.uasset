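; Game instance for Project Dawn that handles save slots, the loading screen and a once-per-second play-time counter.
; SaveGame creates a new SG_PlayerSave, asking through an overwrite widget first if the slot exists.
; SavePlayerData and LoadPlayerData copy hero stats, quests, crafting, inventory, spells, transform and time to and from that object.
; Loading also re-equips gear and relights fast travel points, while AutoSave passes an empty slot name.
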(event Custom|RemoveLoadingScreen
  ;[1 1 1] LoadingScreen
  (bind _loadingscreenref (Variables|Default|GetLoadingScreenRef)
    (:then
      (Widget|RemovefromParent _loadingscreenref))
    (:else)))

(event Custom|CreateLoadingScreen
  ;[1 1 1] LoadingScreen
  (bind _loadingscreenref (Variables|Default|GetLoadingScreenRef)
    (:then
      (Widget|RemovefromParent _loadingscreenref))
    (:else
      _))
  (bind _returnvalue (UserInterface|CreateWidget "/Game/ProjectDawn/Blueprints/HUD/MainMenu/W_LoadingScreen.W_LoadingScreen_C" (Game|GetPlayerController 0)))
  (bind _output_get (Variables|Default|SetLoadingScreenRef _returnvalue))
  (UserInterface|Viewport|AddtoViewport _output_get 0))

(event Custom|ShowMainMenuScreen)

(event Custom|LoadGame
  (params (SaveSlotName :type String))
  (bind _returnvalue (SaveGame|DoesSaveGameExist SaveSlotName))
  (if _returnvalue
    (bind _returnvalue_2 (SaveGame|LoadGamefromSlot SaveSlotName))
    (bind _assg_player_save (Utilities|Casting|CastToSG_PlayerSave _returnvalue_2))
    (Variables|Default|SetSaveGameData _assg_player_save)
    (CallFunction|LoadPlayerData)))

(event Custom|SaveGame
  (params (SlotName :type String))
  (bind _returnvalue (SaveGame|DoesSaveGameExist SlotName))
  (if _returnvalue
    (bind _returnvalue_2 (UserInterface|CreateWidget "/Game/ProjectDawn/Blueprints/HUD/SaveSystem/W_OverwriteSaveData.W_OverwriteSaveData_C"))
    (UserInterface|Viewport|AddtoViewport _returnvalue_2 1)
    (EventDispatchers|BindEventtoOverwriteGameSave _returnvalue_2 (delegate Custom|OverWriteGameSave))
    (else
      (bind _returnvalue_3 (SaveGame|CreateSaveGameObject "/Game/ProjectDawn/Blueprints/Save_Load/SG_PlayerSave.SG_PlayerSave_C"))
      (Variables|Default|SetSaveGameData _returnvalue_3)
      (CallFunction|SavePlayerData SlotName))))

(event Custom|OverWriteGameSave
  (bind _returnvalue (SaveGame|CreateSaveGameObject "/Game/ProjectDawn/Blueprints/Save_Load/SG_PlayerSave.SG_PlayerSave_C"))
  (Variables|Default|SetSaveGameData _returnvalue)
  (CallFunction|SavePlayerData (stale Custom|SaveGame SlotName)))

(event EventInit
  (Utilities|FlowControl|Sequence
    (:then_0
      ;[1 1 1] TimeCounter
      (Math|Integer|IncrementInt (Variables|Default|GetTime) :!label _label
        (:%20%20
          (Utilities|FlowControl|Delay 1.0)
          (goto _label))))))

(fn LoadPlayerData
  (bind _savegamedata (Variables|Default|GetSaveGameData))
  (bind _savegamedata_2 (Variables|Default|GetSaveGameData))
  (Variables|Default|GetSaveGameData
    (:then
      (bind _asbp_hero_base (Utilities|Casting|CastToBP_HeroBase (Game|GetPlayerCharacter 0)))
      (LocalVariables|SetPlayerRef _asbp_hero_base)
      (Utilities|FlowControl|Sequence
        (:then_0
          (Variables|/Game/ProjectDawn/Blueprints/BP_HeroBase.BP_HeroBase_C|SetGold (LocalVariables|GetPlayerRef) (Variables|/Game/ProjectDawn/Blueprints/Save_Load/SG_PlayerSave.SG_PlayerSave_C|GetGold _savegamedata))
          (Default|LoadQuests _savegamedata (Variables|/Game/ProjectDawn/Blueprints/BP_HeroBase.BP_HeroBase_C|GetBC_QuestLogComponent (LocalVariables|GetPlayerRef)))
          (Variables|/Game/ProjectDawn/Blueprints/BP_HeroBase.BP_HeroBase_C|SetPlayerName (LocalVariables|GetPlayerRef) (Variables|/Game/ProjectDawn/Blueprints/Save_Load/SG_PlayerSave.SG_PlayerSave_C|GetPlayerName _savegamedata)))
        (:then_1
          (Variables|/Game/ProjectDawn/Blueprints/BP_HeroBase.BP_HeroBase_C|SetSavePointLocation (LocalVariables|GetPlayerRef) (Variables|/Game/ProjectDawn/Blueprints/Save_Load/SG_PlayerSave.SG_PlayerSave_C|GetLocation _savegamedata)))
        (:then_2
          (Variables|/Game/ProjectDawn/Blueprints/BP_HeroBase.BP_HeroBase_C|SetLevel (LocalVariables|GetPlayerRef) (Variables|/Game/ProjectDawn/Blueprints/Save_Load/SG_PlayerSave.SG_PlayerSave_C|GetLevel _savegamedata))
          (Variables|/Game/ProjectDawn/Blueprints/BP_HeroBase.BP_HeroBase_C|SetCraftingXP (LocalVariables|GetPlayerRef) (Variables|/Game/ProjectDawn/Blueprints/Save_Load/SG_PlayerSave.SG_PlayerSave_C|GetCraftingXP _savegamedata))
          (Variables|/Game/ProjectDawn/Blueprints/BP_HeroBase.BP_HeroBase_C|SetXPReqCraftLevelUp (LocalVariables|GetPlayerRef) (Variables|/Game/ProjectDawn/Blueprints/Save_Load/SG_PlayerSave.SG_PlayerSave_C|GetXPReqCraftLevelUp _savegamedata))
          (Variables|/Game/ProjectDawn/Blueprints/BP_HeroBase.BP_HeroBase_C|SetCraftingList (LocalVariables|GetPlayerRef) (Variables|/Game/ProjectDawn/Blueprints/Save_Load/SG_PlayerSave.SG_PlayerSave_C|GetCraftingList _savegamedata))
          (Variables|/Game/ProjectDawn/Blueprints/BP_HeroBase.BP_HeroBase_C|SetCraftingLevel (LocalVariables|GetPlayerRef) (Variables|/Game/ProjectDawn/Blueprints/Save_Load/SG_PlayerSave.SG_PlayerSave_C|GetCraftingLevel _savegamedata)))
        (:then_3
          (Variables|Default|SetTime (Variables|/Game/ProjectDawn/Blueprints/Save_Load/SG_PlayerSave.SG_PlayerSave_C|GetTime _savegamedata)))
        (:then_4
          (Transformation|SetActorTransform (LocalVariables|GetPlayerRef) (Variables|/Game/ProjectDawn/Blueprints/Save_Load/SG_PlayerSave.SG_PlayerSave_C|GetPlayerTransform _savegamedata))
          (bind _output_get (Variables|/Game/ProjectDawn/Blueprints/BP_HeroBase.BP_HeroBase_C|SetActivatedFastTravelPoints (LocalVariables|GetPlayerRef) (Variables|/Game/ProjectDawn/Blueprints/Save_Load/SG_PlayerSave.SG_PlayerSave_C|GetActivatedFastTravelPoints _savegamedata)))
          (for _array_element _output_get
            (Default|ReLight _array_element)))
        (:then_5
          (Variables|/Game/ProjectDawn/Blueprints/BP_HeroBase.BP_HeroBase_C|SetName (LocalVariables|GetPlayerRef) (Variables|/Game/ProjectDawn/Blueprints/Save_Load/SG_PlayerSave.SG_PlayerSave_C|GetName _savegamedata)))
        (:then_6
          (Variables|/Game/ProjectDawn/Blueprints/BP_HeroBase.BP_HeroBase_C|SetCurrentHealth (LocalVariables|GetPlayerRef) (Variables|/Game/ProjectDawn/Blueprints/Save_Load/SG_PlayerSave.SG_PlayerSave_C|GetCurrentHealth _savegamedata))
          (Variables|/Game/ProjectDawn/Blueprints/BP_HeroBase.BP_HeroBase_C|SetHotBar01 (LocalVariables|GetPlayerRef) (Variables|/Game/ProjectDawn/Blueprints/Save_Load/SG_PlayerSave.SG_PlayerSave_C|GetHotBar01 _savegamedata))
          (Variables|/Game/ProjectDawn/Blueprints/BP_HeroBase.BP_HeroBase_C|SetHotBar02 (LocalVariables|GetPlayerRef) (Variables|/Game/ProjectDawn/Blueprints/Save_Load/SG_PlayerSave.SG_PlayerSave_C|GetHotbar02 _savegamedata)))
        (:then_7
          (Variables|/Game/ProjectDawn/Blueprints/BP_HeroBase.BP_HeroBase_C|SetCurrentMana (LocalVariables|GetPlayerRef) (Variables|/Game/ProjectDawn/Blueprints/Save_Load/SG_PlayerSave.SG_PlayerSave_C|GetCurrentMana _savegamedata)))
        (:then_8
          (Variables|/Game/ProjectDawn/Blueprints/BP_HeroBase.BP_HeroBase_C|SetCurrentXP (LocalVariables|GetPlayerRef) (Variables|/Game/ProjectDawn/Blueprints/Save_Load/SG_PlayerSave.SG_PlayerSave_C|GetCurrentXP _savegamedata)))
        (:then_9
          (Variables|/Game/ProjectDawn/Blueprints/BP_HeroBase.BP_HeroBase_C|SetMaxHealth (LocalVariables|GetPlayerRef) (Variables|/Game/ProjectDawn/Blueprints/Save_Load/SG_PlayerSave.SG_PlayerSave_C|GetMaxHealth _savegamedata)))
        (:then_10
          (Variables|/Game/ProjectDawn/Blueprints/BP_HeroBase.BP_HeroBase_C|SetMaxMana (LocalVariables|GetPlayerRef) (Variables|/Game/ProjectDawn/Blueprints/Save_Load/SG_PlayerSave.SG_PlayerSave_C|GetMaxMana _savegamedata)))
        (:then_11
          (Variables|/Game/ProjectDawn/Blueprints/BP_HeroBase.BP_HeroBase_C|SetXPToNextLevel (LocalVariables|GetPlayerRef) (Variables|/Game/ProjectDawn/Blueprints/Save_Load/SG_PlayerSave.SG_PlayerSave_C|GetXPToNextTevel _savegamedata)))
        (:then_12
          (Variables|/Game/ProjectDawn/Blueprints/BP_HeroBase.BP_HeroBase_C|SetStrength (LocalVariables|GetPlayerRef) (Variables|/Game/ProjectDawn/Blueprints/Save_Load/SG_PlayerSave.SG_PlayerSave_C|GetStrength _savegamedata_2)))
        (:then_13
          (Variables|/Game/ProjectDawn/Blueprints/BP_HeroBase.BP_HeroBase_C|SetDefence (LocalVariables|GetPlayerRef) (Variables|/Game/ProjectDawn/Blueprints/Save_Load/SG_PlayerSave.SG_PlayerSave_C|GetDefence _savegamedata_2)))
        (:then_14
          (bind _output_get_2 (Variables|/Game/ProjectDawn/Blueprints/BP_HeroBase.BP_HeroBase_C|SetSwordInfo (LocalVariables|GetPlayerRef) (Variables|/Game/ProjectDawn/Blueprints/Save_Load/SG_PlayerSave.SG_PlayerSave_C|GetSwordInfo _savegamedata_2)))
          (if (Utilities|IsValidClass (.ItemClass (Utilities|Struct|BreakDS_ItemInfo _output_get_2)))
            (Default|UnequipGear (LocalVariables|GetPlayerRef) :!label _label)
            (Default|EquipGear (LocalVariables|GetPlayerRef))))
        (:then_15
          (bind _output_get_3 (Variables|/Game/ProjectDawn/Blueprints/BP_HeroBase.BP_HeroBase_C|SetShieldInfo (LocalVariables|GetPlayerRef) (Variables|/Game/ProjectDawn/Blueprints/Save_Load/SG_PlayerSave.SG_PlayerSave_C|GetShieldInfo _savegamedata_2)))
          (if (Utilities|IsValidClass (.ItemClass (Utilities|Struct|BreakDS_ItemInfo _output_get_3)))
            (goto _label)))
        (:then_16
          (bind _output_get_4 (Variables|/Game/ProjectDawn/Blueprints/BP_HeroBase.BP_HeroBase_C|SetAccesoryInfo (LocalVariables|GetPlayerRef) (Variables|/Game/ProjectDawn/Blueprints/Save_Load/SG_PlayerSave.SG_PlayerSave_C|GetAccessoryInfo _savegamedata_2)))
          (if (Utilities|IsValidClass (.ItemClass (Utilities|Struct|BreakDS_ItemInfo _output_get_4)))
            (goto _label)))
        (:then_17
          (bind _output_get_5 (Variables|/Game/ProjectDawn/Blueprints/BP_HeroBase.BP_HeroBase_C|SetBowInfo (LocalVariables|GetPlayerRef) (Variables|/Game/ProjectDawn/Blueprints/Save_Load/SG_PlayerSave.SG_PlayerSave_C|GetBowInfo _savegamedata_2)))
          (if (Utilities|IsValidClass (.ItemClass (Utilities|Struct|BreakDS_ItemInfo _output_get_5)))
            (goto _label)))
        (:then_18
          (Variables|/Game/ProjectDawn/Blueprints/BP_HeroBase.BP_HeroBase_C|SetArrowInfo (LocalVariables|GetPlayerRef) (Variables|/Game/ProjectDawn/Blueprints/Save_Load/SG_PlayerSave.SG_PlayerSave_C|GetArrowInfo _savegamedata_2)))
        (:then_19
          (Variables|/Game/ProjectDawn/Blueprints/BP_HeroBase.BP_HeroBase_C|SetInventory (LocalVariables|GetPlayerRef) (Variables|/Game/ProjectDawn/Blueprints/Save_Load/SG_PlayerSave.SG_PlayerSave_C|GetInventory _savegamedata_2)))
        (:then_20
          (Variables|/Game/ProjectDawn/Blueprints/BP_HeroBase.BP_HeroBase_C|SetInventorySize (LocalVariables|GetPlayerRef) (Variables|/Game/ProjectDawn/Blueprints/Save_Load/SG_PlayerSave.SG_PlayerSave_C|GetInventorySize _savegamedata_2)))
        (:then_21
          (Variables|/Game/ProjectDawn/Blueprints/BP_HeroBase.BP_HeroBase_C|SetSpellSelected (LocalVariables|GetPlayerRef) (Variables|/Game/ProjectDawn/Blueprints/Save_Load/SG_PlayerSave.SG_PlayerSave_C|GetSpellSelected _savegamedata_2)))
        (:then_22
          (Variables|/Game/ProjectDawn/Blueprints/BP_HeroBase.BP_HeroBase_C|SetSpellsKnown (LocalVariables|GetPlayerRef) (Variables|/Game/ProjectDawn/Blueprints/Save_Load/SG_PlayerSave.SG_PlayerSave_C|GetSpellsKnown _savegamedata_2)))))
    (:else)))

(fn SavePlayerData
  (params (SaveSlotName :type String))
  (bind _savegamedata (Variables|Default|GetSaveGameData))
  (bind _asbp_hero_base (Utilities|Casting|CastToBP_HeroBase (Game|GetPlayerCharacter 0)))
  (LocalVariables|SetPlayerRef _asbp_hero_base)
  (Utilities|FlowControl|Sequence
    (:then_0
      (Variables|/Game/ProjectDawn/Blueprints/Save_Load/SG_PlayerSave.SG_PlayerSave_C|SetLocation _savegamedata (Variables|/Game/ProjectDawn/Blueprints/BP_HeroBase.BP_HeroBase_C|GetSavePointLocation (LocalVariables|GetPlayerRef)))
      (for _array_element (Variables|/Game/ProjectDawn/Blueprints/Quest/New/BC_QuestLogComponent.BC_QuestLogComponent_C|GetCurrentQuests (Variables|/Game/ProjectDawn/Blueprints/BP_HeroBase.BP_HeroBase_C|GetBC_QuestLogComponent (LocalVariables|GetPlayerRef)))
        (Default|SaveQuestDetails _savegamedata _array_element))
      (Default|SaveQuestLog _savegamedata (Variables|/Game/ProjectDawn/Blueprints/BP_HeroBase.BP_HeroBase_C|GetBC_QuestLogComponent (LocalVariables|GetPlayerRef)))
      (Variables|/Game/ProjectDawn/Blueprints/Save_Load/SG_PlayerSave.SG_PlayerSave_C|SetPlayerName _savegamedata (Variables|/Game/ProjectDawn/Blueprints/BP_HeroBase.BP_HeroBase_C|GetPlayerName (LocalVariables|GetPlayerRef))))
    (:then_1
      (Variables|/Game/ProjectDawn/Blueprints/Save_Load/SG_PlayerSave.SG_PlayerSave_C|SetLevel _savegamedata (Variables|/Game/ProjectDawn/Blueprints/BP_HeroBase.BP_HeroBase_C|GetLevel (LocalVariables|GetPlayerRef))))
    (:then_2
      (Variables|/Game/ProjectDawn/Blueprints/Save_Load/SG_PlayerSave.SG_PlayerSave_C|SetGold _savegamedata (Variables|/Game/ProjectDawn/Blueprints/BP_HeroBase.BP_HeroBase_C|GetGold (LocalVariables|GetPlayerRef)))
      (Variables|/Game/ProjectDawn/Blueprints/Save_Load/SG_PlayerSave.SG_PlayerSave_C|SetCraftingXP _savegamedata (Variables|/Game/ProjectDawn/Blueprints/BP_HeroBase.BP_HeroBase_C|GetCraftingXP (LocalVariables|GetPlayerRef)))
      (Variables|/Game/ProjectDawn/Blueprints/Save_Load/SG_PlayerSave.SG_PlayerSave_C|SetXPReqCraftLevelUp _savegamedata (Variables|/Game/ProjectDawn/Blueprints/BP_HeroBase.BP_HeroBase_C|GetXPReqCraftLevelUp (LocalVariables|GetPlayerRef)))
      (Variables|/Game/ProjectDawn/Blueprints/Save_Load/SG_PlayerSave.SG_PlayerSave_C|SetCraftingLevel _savegamedata (Variables|/Game/ProjectDawn/Blueprints/BP_HeroBase.BP_HeroBase_C|GetCraftingLevel (LocalVariables|GetPlayerRef)))
      (Variables|/Game/ProjectDawn/Blueprints/Save_Load/SG_PlayerSave.SG_PlayerSave_C|SetCraftingList _savegamedata (Variables|/Game/ProjectDawn/Blueprints/BP_HeroBase.BP_HeroBase_C|GetCraftingList (LocalVariables|GetPlayerRef))))
    (:then_3
      (Variables|/Game/ProjectDawn/Blueprints/Save_Load/SG_PlayerSave.SG_PlayerSave_C|SetPlayerTransform _savegamedata (Transformation|GetActorTransform (LocalVariables|GetPlayerRef))))
    (:then_4
      (Variables|/Game/ProjectDawn/Blueprints/Save_Load/SG_PlayerSave.SG_PlayerSave_C|SetTime _savegamedata (Variables|Default|GetTime))
      (Variables|/Game/ProjectDawn/Blueprints/Save_Load/SG_PlayerSave.SG_PlayerSave_C|SetActivatedFastTravelPoints _savegamedata (Variables|/Game/ProjectDawn/Blueprints/BP_HeroBase.BP_HeroBase_C|GetActivatedFastTravelPoints (LocalVariables|GetPlayerRef)))
      (Variables|/Game/ProjectDawn/Blueprints/Save_Load/SG_PlayerSave.SG_PlayerSave_C|SetHotBar01 _savegamedata (Variables|/Game/ProjectDawn/Blueprints/BP_HeroBase.BP_HeroBase_C|GetHotBar01 (LocalVariables|GetPlayerRef)))
      (Variables|/Game/ProjectDawn/Blueprints/Save_Load/SG_PlayerSave.SG_PlayerSave_C|SetHotbar02 _savegamedata (Variables|/Game/ProjectDawn/Blueprints/BP_HeroBase.BP_HeroBase_C|GetHotBar02 (LocalVariables|GetPlayerRef))))
    (:then_5
      (Variables|/Game/ProjectDawn/Blueprints/Save_Load/SG_PlayerSave.SG_PlayerSave_C|SetName _savegamedata (Variables|/Game/ProjectDawn/Blueprints/BP_HeroBase.BP_HeroBase_C|GetName (LocalVariables|GetPlayerRef))))
    (:then_6
      (Variables|/Game/ProjectDawn/Blueprints/Save_Load/SG_PlayerSave.SG_PlayerSave_C|SetCurrentHealth _savegamedata (Variables|/Game/ProjectDawn/Blueprints/BP_HeroBase.BP_HeroBase_C|GetCurrentHealth (LocalVariables|GetPlayerRef))))
    (:then_7
      (Variables|/Game/ProjectDawn/Blueprints/Save_Load/SG_PlayerSave.SG_PlayerSave_C|SetCurrentMana _savegamedata (Variables|/Game/ProjectDawn/Blueprints/BP_HeroBase.BP_HeroBase_C|GetCurrentMana (LocalVariables|GetPlayerRef))))
    (:then_8
      (Variables|/Game/ProjectDawn/Blueprints/Save_Load/SG_PlayerSave.SG_PlayerSave_C|SetCurrentXP _savegamedata (Variables|/Game/ProjectDawn/Blueprints/BP_HeroBase.BP_HeroBase_C|GetCurrentXP (LocalVariables|GetPlayerRef))))
    (:then_9
      (Variables|/Game/ProjectDawn/Blueprints/Save_Load/SG_PlayerSave.SG_PlayerSave_C|SetMaxHealth _savegamedata (Variables|/Game/ProjectDawn/Blueprints/BP_HeroBase.BP_HeroBase_C|GetMaxHealth (LocalVariables|GetPlayerRef))))
    (:then_10
      (Variables|/Game/ProjectDawn/Blueprints/Save_Load/SG_PlayerSave.SG_PlayerSave_C|SetMaxMana _savegamedata (Variables|/Game/ProjectDawn/Blueprints/BP_HeroBase.BP_HeroBase_C|GetMaxMana (LocalVariables|GetPlayerRef))))
    (:then_11
      (Variables|/Game/ProjectDawn/Blueprints/Save_Load/SG_PlayerSave.SG_PlayerSave_C|SetXPToNextTevel _savegamedata (Variables|/Game/ProjectDawn/Blueprints/BP_HeroBase.BP_HeroBase_C|GetXPToNextLevel (LocalVariables|GetPlayerRef))))
    (:then_12
      (Variables|/Game/ProjectDawn/Blueprints/Save_Load/SG_PlayerSave.SG_PlayerSave_C|SetStrength _savegamedata (Variables|/Game/ProjectDawn/Blueprints/BP_HeroBase.BP_HeroBase_C|GetStrength (LocalVariables|GetPlayerRef))))
    (:then_13
      (Variables|/Game/ProjectDawn/Blueprints/Save_Load/SG_PlayerSave.SG_PlayerSave_C|SetDefence _savegamedata (Variables|/Game/ProjectDawn/Blueprints/BP_HeroBase.BP_HeroBase_C|GetDefence (LocalVariables|GetPlayerRef))))
    (:then_14
      (Variables|/Game/ProjectDawn/Blueprints/Save_Load/SG_PlayerSave.SG_PlayerSave_C|SetSwordInfo _savegamedata (Variables|/Game/ProjectDawn/Blueprints/BP_HeroBase.BP_HeroBase_C|GetSwordInfo (LocalVariables|GetPlayerRef))))
    (:then_15
      (Variables|/Game/ProjectDawn/Blueprints/Save_Load/SG_PlayerSave.SG_PlayerSave_C|SetShieldInfo _savegamedata (Variables|/Game/ProjectDawn/Blueprints/BP_HeroBase.BP_HeroBase_C|GetShieldInfo (LocalVariables|GetPlayerRef))))
    (:then_16
      (Variables|/Game/ProjectDawn/Blueprints/Save_Load/SG_PlayerSave.SG_PlayerSave_C|SetAccessoryInfo _savegamedata (Variables|/Game/ProjectDawn/Blueprints/BP_HeroBase.BP_HeroBase_C|GetAccesoryInfo (LocalVariables|GetPlayerRef))))
    (:then_17
      (Variables|/Game/ProjectDawn/Blueprints/Save_Load/SG_PlayerSave.SG_PlayerSave_C|SetBowInfo _savegamedata (Variables|/Game/ProjectDawn/Blueprints/BP_HeroBase.BP_HeroBase_C|GetBowInfo (LocalVariables|GetPlayerRef))))
    (:then_18
      (Variables|/Game/ProjectDawn/Blueprints/Save_Load/SG_PlayerSave.SG_PlayerSave_C|SetArrowInfo _savegamedata (Variables|/Game/ProjectDawn/Blueprints/BP_HeroBase.BP_HeroBase_C|GetArrowInfo (LocalVariables|GetPlayerRef))))
    (:then_19
      (Variables|/Game/ProjectDawn/Blueprints/Save_Load/SG_PlayerSave.SG_PlayerSave_C|SetInventory _savegamedata (Variables|/Game/ProjectDawn/Blueprints/BP_HeroBase.BP_HeroBase_C|GetInventory (LocalVariables|GetPlayerRef))))
    (:then_20
      (Variables|/Game/ProjectDawn/Blueprints/Save_Load/SG_PlayerSave.SG_PlayerSave_C|SetInventorySize _savegamedata (Variables|/Game/ProjectDawn/Blueprints/BP_HeroBase.BP_HeroBase_C|GetInventorySize (LocalVariables|GetPlayerRef))))
    (:then_21
      (Variables|/Game/ProjectDawn/Blueprints/Save_Load/SG_PlayerSave.SG_PlayerSave_C|SetSpellSelected _savegamedata (Variables|/Game/ProjectDawn/Blueprints/BP_HeroBase.BP_HeroBase_C|GetSpellSelected (LocalVariables|GetPlayerRef))))
    (:then_22
      (Variables|/Game/ProjectDawn/Blueprints/Save_Load/SG_PlayerSave.SG_PlayerSave_C|SetSpellsKnown _savegamedata (Variables|/Game/ProjectDawn/Blueprints/BP_HeroBase.BP_HeroBase_C|GetSpellsKnown (LocalVariables|GetPlayerRef)))
      (SaveGame|SaveGametoSlot _savegamedata SaveSlotName))))

(fn ClearSaveData
  (SaveGame|DeleteGameinSlot (Variables|Default|GetSaveSlotName)))

(fn AutoSave
  (CallFunction|SavePlayerData))