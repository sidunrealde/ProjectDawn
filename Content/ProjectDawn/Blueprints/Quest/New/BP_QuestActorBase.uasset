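; Base quest actor that tracks objective progress for one quest, loading its current stage from DT_QuestData.
; It listens to the hero's objective-ID events and pre-counts inventory items for one objective type on BeginPlay.
; Completed objectives show a notification, play a sound and grant bonus XP and items.
; Finished stages advance to the next or mark the quest completed, with auto-complete quests turned in through the player's BC_QuestLogComponent.
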(event EventBeginPlay
  (Utilities|FlowControl|Sequence
    (:then_0
      (CallFunction|GetQuestDetails)
      (EventDispatchers|BindEventtoOnObjectiveIDCalled (CallFunction|GetHeroCharacter) (EventDispatchers|CreateEvent :!event OnObjectiveIDHeard))
      (for _array_element (.Objectives (Utilities|Struct|BreakDS_QuestStageDetails (Variables|Default|GetCurrentStageDetails)))
        (if (Utilities|Enum|Equal(Enum) (.Type (Utilities|Struct|BreakDS_ObjectiveDetails _array_element)) "NewEnumerator3")
          (for _array_element_2 (Variables|/Game/ProjectDawn/Blueprints/BP_HeroBase.BP_HeroBase_C|GetInventory (CallFunction|GetHeroCharacter))
            (if (Utilities|Enum|Equal(Enum) (.ItemName (Utilities|Struct|BreakDS_ItemInfo _array_element_2)) (Utilities|Text|ToText(String) (.ObjectiveID (Utilities|Struct|BreakDS_ObjectiveDetails _array_element))))
              (Variables|Default|SetCollectItemsHeld (+ (.CurrentStack (Utilities|Struct|BreakDS_ItemInfo _array_element_2)) (Variables|Default|GetCollectItemsHeld)))))
          (CallFunction|OnObjectiveIDHeard (.ObjectiveID (Utilities|Struct|BreakDS_ObjectiveDetails _array_element)) (Variables|Default|GetCollectItemsHeld)))))
    (:then_1
      (Utilities|FlowControl|Delay 1.0)
      (bind _return (CallFunction|AreAllObjectivesComplete))
      (Variables|Default|SetIsCompleted _return))))

(fn ConstructionScript)

(fn OnObjectiveIDHeard
  (params (ObjectiveID :type String) (Value :type Integer))
  (bind _currentobjectiveprogress (Variables|Default|GetCurrentObjectiveProgress))
  (bind (_value _returnvalue) (Utilities|Map|Find _currentobjectiveprogress ObjectiveID))
  (if (> (Class|KismetMathLibrary|SignOfInteger Value) 0)
    (if _returnvalue
      (if (> (Utilities|Struct|BreakDS_ObjectiveDetails (CallFunction|GetObjectiveDatabyID ObjectiveID)) _value)
        (Utilities|Map|Add (Variables|Default|GetCurrentObjectiveProgress) ObjectiveID (+ _value Value))
        (CallFunction|IsObjectiveComplete ObjectiveID)
        (Default|CallOnObjectiveHeard)
        (return))
      (else
        (return)))
    (else
      (Utilities|Map|Add (Variables|Default|GetCurrentObjectiveProgress) ObjectiveID (+ (.Value (Utilities|Map|Find (Variables|Default|GetCurrentObjectiveProgress) ObjectiveID)) Value))
      (return))))

(fn GetQuestDetails
  (bind _currentobjectiveprogress (Variables|Default|GetCurrentObjectiveProgress))
  (bind _returnvalue (Utilities|GetDataTableRow "/Game/ProjectDawn/Blueprints/Quest/New/DT_QuestData.DT_QuestData" (Variables|Default|GetQuestID))
    (:then
      (bind _output_get (Variables|Default|SetQuestDetails _returnvalue))
      (bind _output_get_2 (Variables|Default|SetCurrentStageDetails (Utilities|Array|Get(acopy) (.Stages (Utilities|Struct|BreakDS_QuestDetails _output_get)) (Variables|Default|GetCurrentStage))))
      (Utilities|Map|Clear _currentobjectiveprogress)
      (for _array_element (.Objectives (Utilities|Struct|BreakDS_QuestStageDetails _output_get_2))
        (Utilities|Map|Add _currentobjectiveprogress (.ObjectiveID (Utilities|Struct|BreakDS_ObjectiveDetails _array_element)) 0)))))

(fn GetObjectiveDatabyID
  (params (ObjectiveID :type String))
  (for _array_element (.Objectives (Utilities|Struct|BreakDS_QuestStageDetails (Variables|Default|GetCurrentStageDetails)))
    (if (Utilities|Enum|Equal(Enum) (Utilities|Struct|BreakDS_ObjectiveDetails _array_element) ObjectiveID)
      (return _array_element))))

(fn IsObjectiveComplete
  (params (ObjectiveID :type String))
  (bind _currentobjective (CallFunction|GetObjectiveDatabyID ObjectiveID))
  (bind _herocharacter (CallFunction|GetHeroCharacter))
  (bind (_description _quantity) (Utilities|Struct|BreakDS_ObjectiveDetails _currentobjective))
  (bind _currentobjective_2 (CallFunction|GetObjectiveDatabyID ObjectiveID))
  (bind (_bonusxp _bonusitemrewards) (Utilities|Struct|BreakDS_ObjectiveDetails _currentobjective_2))
  (if (>= (.Value (Utilities|Map|Find (Variables|Default|GetCurrentObjectiveProgress) ObjectiveID)) _quantity)
    (bind _returnvalue (UserInterface|CreateWidget "/Game/ProjectDawn/Blueprints/HUD/Quest/W_QuestNotification.W_QuestNotification_C" 0 _description))
    (UserInterface|Viewport|AddtoViewport _returnvalue 0)
    (Audio|PlaySound2D "/Game/ProjectDawn/Blueprints/Sounds/AC_ObjectiveComplete.AC_ObjectiveComplete" 1.0 1.0 0.0 0 0)
    (bind _return (CallFunction|AreAllObjectivesComplete))
    (if _return
      (bind _result (Math|Integer|IncrementInt (Variables|Default|GetCurrentStage))
        (:%20%20
          (if (Utilities|Array|IsValidIndex (Utilities|Struct|BreakDS_QuestDetails (Variables|Default|GetQuestDetails)) _result)
            (CallFunction|GetQuestDetails)
            (else
              (Variables|Default|SetIsCompleted true))))))
    (Default|GainXP _herocharacter _bonusxp)
    (bind _keys (Utilities|Map|Keys _bonusitemrewards))
    (bind _values (Utilities|Map|Values _bonusitemrewards))
    (for (_array_element _array_index) _keys
      (bind _returnvalue_2 (Utilities|GetDataTableRow "/Game/ProjectDawn/Blueprints/Items/Data/DT_ItemInfo.DT_ItemInfo" (Utilities|String|StringToName (Utilities|String|EnumtoString _array_element)))
        (:then
          (for _index (range 0 (- (Utilities|Array|Get(acopy) _values _array_index) 1))
            (Default|PickupItem _herocharacter _returnvalue_2)))))))

(fn AreAllObjectivesComplete
  (for _array_element (.Objectives (Utilities|Struct|BreakDS_QuestStageDetails (Variables|Default|GetCurrentStageDetails)))
    (if (not (>= (.Value (Utilities|Map|Find (Variables|Default|GetCurrentObjectiveProgress) (Utilities|Struct|BreakDS_ObjectiveDetails _array_element))) (.Quantity (Utilities|Struct|BreakDS_ObjectiveDetails (CallFunction|GetObjectiveDatabyID (Utilities|Struct|BreakDS_ObjectiveDetails _array_element))))))
      (bind _output_get (LocalVariables|SetLocal_AreAllComplete false))
      (return _output_get)))
  (if (and (Utilities|Struct|BreakDS_QuestDetails (Variables|Default|GetQuestDetails)) (LocalVariables|GetLocal_AreAllComplete))
    (Default|TurninQuest (Actor|GetComponentbyClass (Game|GetPlayerCharacter 0) "/Game/ProjectDawn/Blueprints/Quest/New/BC_QuestLogComponent.BC_QuestLogComponent_C") (Variables|Default|GetQuestID)))
  (return (LocalVariables|GetLocal_AreAllComplete)))

(fn AreAllStagesComplete
  (Utilities|FlowControl|ForLoopwithBreak 0 (- (Utilities|Array|Length (.Stages (Utilities|Struct|BreakDS_QuestDetails (Variables|Default|GetQuestDetails)))) 1) :!label _label
    (:LoopBody
      (CallFunction|GetQuestDetails)
      (bind _return (CallFunction|AreAllObjectivesComplete))
      (if _return
        (Math|Integer|IncrementInt (Variables|Default|GetCurrentStage))
        (else
          (LocalVariables|SetAllStagesComplete false)
          (goto _label Break))))))