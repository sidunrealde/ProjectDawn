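; Quest NPC for Quest 004 that ties its dialogue component to the quest giver component for offering a quest and handing out rewards.
; On interaction it checks the hero's quest log, selects the turn-in dialogue if the quest awaits turn-in, then opens the conversation.
; Dialogue events display the quest or rewards widget, whose accept and decline callbacks switch dialogue trees, clear progress and end the talking state.
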(event Custom|QuestTurnInWidgetDisplay
  (bind _bc_questgivercomponent (Variables|Default|GetBC_QuestGiverComponent))
  (bind _questrewardswidgetref (Variables|/Game/ProjectDawn/Blueprints/Quest/New/BC_QuestGiverComponent.BC_QuestGiverComponent_C|GetQuestRewardsWidgetRef _bc_questgivercomponent))
  (Default|DisplayRewards _bc_questgivercomponent)
  (EventDispatchers|BindEventtoOnRewardsAccept _questrewardswidgetref (delegate Custom|AcceptRewards))
  (EventDispatchers|BindEventtoOnRewardsDecline _questrewardswidgetref (delegate Custom|DeclineRewards)))

(event Custom|AcceptRewards
  (bind _bcc_dialoguequestnpc_004 (Variables|Default|GetBCC_DialogueQuestNPC_004))
  (Variables|Default|SetIsTalking false)
  (Default|SetDialogueTreeIndex _bcc_dialoguequestnpc_004 1)
  (Default|ClearDialogueProgress _bcc_dialoguequestnpc_004))

(event Custom|DeclineRewards
  (bind _bcc_dialoguequestnpc_004 (Variables|Default|GetBCC_DialogueQuestNPC_004))
  (Variables|Default|SetIsTalking false)
  (Default|SetDialogueTreeIndex _bcc_dialoguequestnpc_004 2)
  (Default|ClearDialogueProgress _bcc_dialoguequestnpc_004))

(event Custom|QuestWidgetDisplay
  (bind _bc_questgivercomponent (Variables|Default|GetBC_QuestGiverComponent))
  (bind _questgiverwidgetref (Variables|/Game/ProjectDawn/Blueprints/Quest/New/BC_QuestGiverComponent.BC_QuestGiverComponent_C|GetQuestGiverWidgetRef _bc_questgivercomponent))
  (Default|DisplayQuest (Variables|Default|GetBC_QuestGiverComponent))
  (Utilities|IsValid _questgiverwidgetref
    (:Is%20Valid
      (EventDispatchers|BindEventtoOnQuestAccept _questgiverwidgetref (delegate Custom|QuestAcceptEvent))
      (EventDispatchers|BindEventtoOnQuestDecline _questgiverwidgetref (delegate Custom|QuestDeclineEvent)))))

(event Custom|QuestAcceptEvent
  (bind _bcc_dialoguequestnpc_004 (Variables|Default|GetBCC_DialogueQuestNPC_004))
  (Variables|Default|SetIsTalking false)
  (Default|SetDialogueTreeIndex _bcc_dialoguequestnpc_004 1)
  (Default|ClearDialogueProgress _bcc_dialoguequestnpc_004))

(event Custom|QuestDeclineEvent
  (bind _bcc_dialoguequestnpc_004 (Variables|Default|GetBCC_DialogueQuestNPC_004))
  (Variables|Default|SetIsTalking false)
  (Default|SetDialogueTreeIndex _bcc_dialoguequestnpc_004 2)
  (Default|ClearDialogueProgress _bcc_dialoguequestnpc_004))

(event Custom|ResetTalkState
  (Variables|Default|SetIsTalking false))

(event EventBeginPlay
  (|CallParentFunction)
  (Utilities|FlowControl|Sequence
    (:then_0
      (Variables|/Game/ProjectDawn/Blueprints/Dialogue/BC_DialogueBaseComponent.BC_DialogueBaseComponent_C|SetNPCRef (Variables|Default|GetBCC_DialogueQuestNPC_004) self)
      (EventDispatchers|BindEventtoOnQuestGiverWidget (Variables|Default|GetBCC_DialogueQuestNPC_004) (delegate Custom|QuestWidgetDisplay)))
    (:then_1
      (EventDispatchers|BindEventtoOnQuestTurninWidget (Variables|Default|GetBCC_DialogueQuestNPC_004) (delegate Custom|QuestTurnInWidgetDisplay))
      (EventDispatchers|BindEventtoOnConversationClosed (Variables|Default|GetBCC_DialogueQuestNPC_004) (delegate Custom|ResetTalkState)))))

(fn ConstructionScript
  (|CallParentFunction))

(fn QuestInteract
  (bind _questactor (Default|GetQuestActor (Variables|/Game/ProjectDawn/Blueprints/BP_HeroBase.BP_HeroBase_C|GetBC_QuestLogComponent (CallFunction|GetHeroCharacter)) (.rowname (Variables|/Game/ProjectDawn/Blueprints/Quest/New/BC_QuestGiverComponent.BC_QuestGiverComponent_C|GetQuestData (Variables|Default|GetBC_QuestGiverComponent)))))
  (Utilities|IsValid _questactor
    (:Is%20Valid
      (if (and (Variables|/Game/ProjectDawn/Blueprints/Quest/New/BP_QuestActorBase.BP_QuestActorBase_C|GetIsCompleted _questactor) (not (Variables|/Game/ProjectDawn/Blueprints/Quest/New/BP_QuestActorBase.BP_QuestActorBase_C|GetIsTurnedIn _questactor)))
        (Default|SetDialogueTreeIndex (Variables|Default|GetBCC_DialogueQuestNPC_004) 3)))
    (:Is%20Not%20Valid
      _))
  (CallFunction|ReadyDialoguePlayerCamera)
  (Default|OpenConversation (Variables|Default|GetBCC_DialogueQuestNPC_004))
  (Variables|Default|SetIsTalking true)
  (Default|QuestInteract (Variables|Default|GetBC_QuestGiverComponent))
  (return (Variables|Default|GetObjective%20ID)))