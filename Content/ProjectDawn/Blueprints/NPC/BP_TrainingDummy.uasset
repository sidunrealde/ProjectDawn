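; Training dummy NPC that shows elemental status effects with particle emitters attached to its mesh.
; The elemental effect event always sets the burning status and stores the spawned fire emitter.
; Freeze only takes hold on a burning dummy with a valid fire emitter, which it destroys and replaces with a frost emitter.
; Shock, damage handling and EnemyRef are empty stubs, with a shock emitter left unconnected.
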(event Custom|Freeze_1
  (bind _burning (Variables|Default|GetBurning))
  (if (Utilities|Enum|Equal(Enum) (Variables|Default|GetStatusEffect) "NewEnumerator1")
    (Utilities|IsValid _burning
      (:Is%20Valid
        (Components|DestroyComponent _burning)
        (Variables|Default|SetStatusEffect "NewEnumerator2")
        (bind _returnvalue (Effects|SpawnEmitterAttached "/Game/InfinityBladeEffects/Effects/FX_Mobile/ICE/combat/P_Buff_ShoutFreeze_02.P_Buff_ShoutFreeze_02" (Variables|Character|GetMesh) "None" "0, 0, 0" "0, 0, 0" "1.000000,1.000000,1.000000" "SnapToTargetIncludingScale"))
        (Variables|Default|SetFrozen _returnvalue)))
    (elif (Utilities|Enum|Equal(Enum) (Variables|Default|GetStatusEffect) "NewEnumerator3")
      _)))

(event Custom|Shock_1)

(event EventElementalEffect
  (params (Potency :type Float%20%28double-precision%29) (SpellType :type EN_SpellType%20Enum :default "NewEnumerator0") (ElementalType :type EN_ElementalTypes%20Enum :default "NewEnumerator0"))
  (Variables|Default|SetStatusEffect "NewEnumerator1")
  (bind _returnvalue (Effects|SpawnEmitterAttached "/Game/InfinityBladeEffects/Effects/FX_Mobile/Fire/combat/P_Buff_JumpDiveFire_02.P_Buff_JumpDiveFire_02" (Variables|Character|GetMesh) "None" "0, 0, 0" "0, 0, 0" "1.000000,1.000000,1.000000" "SnapToTargetIncludingScale"))
  (Variables|Default|SetBurning _returnvalue))

(event Game|Damage|EventAnyDamage
  (params (Damage :type Float%20%28single-precision%29) (DamageType :type Damage%20Type%20Object%20Reference) (InstigatedBy :type Controller%20Object%20Reference) (DamageCauser :type Actor%20Object%20Reference)))

(fn ConstructionScript)

(fn EnemyRef
  (return 0))