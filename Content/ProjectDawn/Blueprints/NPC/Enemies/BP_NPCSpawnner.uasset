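; NPC enemy spawner that keeps a capped population of random enemy types near player 0.
; A self-repeating delayed check prunes dead units, spawns one inside SpawnZone, or destroys all when the player leaves activation range.
; After spawning, a downward trace moves the spawner itself, not the new unit, to the ground hit.
; Heroes inside ShutoffZone pause spawning; the construction script sizes both zones.
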(event OnComponentBeginOverlap(ShutoffZone)
  (params (OverlappedComponent :type Primitive%20Component%20Object%20Reference) (OtherActor :type Actor%20Object%20Reference) (OtherComp :type Primitive%20Component%20Object%20Reference) (OtherBodyIndex :type Integer) (bFromSweep :type Boolean) (SweepResult :type Hit%20Result%20Structure%20%28by%20ref%29))
  (Utilities|Casting|CastToBP_HeroBase OtherActor)
  (Variables|Default|SetIsActive false))

(event OnComponentEndOverlap(ShutoffZone)
  (params (OverlappedComponent :type Primitive%20Component%20Object%20Reference) (OtherActor :type Actor%20Object%20Reference) (OtherComp :type Primitive%20Component%20Object%20Reference) (OtherBodyIndex :type Integer))
  (Utilities|Casting|CastToBP_HeroBase OtherActor)
  (Variables|Default|SetIsActive true))

(event Custom|SpawnCheck
  (bind _spawnzone (Variables|Default|GetSpawnZone))
  (if (> (Variables|Default|GetSpawnnerActivationDistance) (Transformation|GetDistanceTo (Game|GetPlayerCharacter 0)))
    (if (Variables|Default|GetIsActive)
      (for _array_element (Variables|Default|GetSpawnedUnits)
        (Utilities|IsValid _array_element
          (:Is%20Not%20Valid
            (Utilities|Array|RemoveItem (Variables|Default|GetSpawnedUnits) _array_element))))
      (if (>= (Utilities|Array|Length (Variables|Default|GetSpawnedUnits)) (Variables|Default|GetNumberOfEnemies))
        _
        (else
          (bind _returnvalue (Game|SpawnActorfromClass (.OutItem (Utilities|Array|Random (Variables|Default|GetEnemiesToSpawn))) (Math|Transform|MakeTransform (Math|Random|RandomPointinBoundingBox (Transformation|GetWorldLocation _spawnzone) (/ (Components|Box|GetScaledBoxExtent _spawnzone) 2.0)) (Math|Rotator|MakeRotator 0.0 0.0 (Math|Random|RandomFloatinRange -1.8e+02 1.8e+02)) "1.000000,1.000000,1.000000") "Undefined" "SelectDefaultAtRuntime" 0 0))
          (Utilities|IsValid _returnvalue
            (:Is%20Valid
              (Utilities|Array|AddUnique (Variables|Default|GetSpawnedUnits) _returnvalue)
              (bind (_outhit _returnvalue_2) (Collision|LineTraceByChannel (Transformation|GetActorLocation _returnvalue) (- (Transformation|GetActorLocation _returnvalue) "0.000000,0.000000,2000.000000") "TraceTypeQuery1" false (Utilities|Array|MakeArray _returnvalue) "None"))
              (if _returnvalue_2
                (Transformation|SetActorLocation (.Location (Collision|BreakHitResult _outhit)) false false)))
            (:Is%20Not%20Valid
              _)))))
    (else
      (for _array_element_2 (Variables|Default|GetSpawnedUnits)
        (Actor|DestroyActor _array_element_2))
      (Variables|Default|SetSpawnedUnits (Utilities|Array|MakeArray))))
  (Utilities|FlowControl|Delay (Variables|Default|GetSpawnDelay))
  (CallFunction|SpawnCheck))

(event EventBeginPlay
  (bind _spawnzone (Variables|Default|GetSpawnZone))
  (if (> (Variables|Default|GetSpawnnerActivationDistance) (Transformation|GetDistanceTo (Game|GetPlayerCharacter 0)))
    (if (Variables|Default|GetIsActive)
      (for _array_element (Variables|Default|GetSpawnedUnits)
        (Utilities|IsValid _array_element
          (:Is%20Not%20Valid
            (Utilities|Array|RemoveItem (Variables|Default|GetSpawnedUnits) _array_element))))
      (if (>= (Utilities|Array|Length (Variables|Default|GetSpawnedUnits)) (Variables|Default|GetNumberOfEnemies))
        _
        (else
          (bind _returnvalue (Game|SpawnActorfromClass (.OutItem (Utilities|Array|Random (Variables|Default|GetEnemiesToSpawn))) (Math|Transform|MakeTransform (Math|Random|RandomPointinBoundingBox (Transformation|GetWorldLocation _spawnzone) (/ (Components|Box|GetScaledBoxExtent _spawnzone) 2.0)) (Math|Rotator|MakeRotator 0.0 0.0 (Math|Random|RandomFloatinRange -1.8e+02 1.8e+02)) "1.000000,1.000000,1.000000") "Undefined" "SelectDefaultAtRuntime" 0 0))
          (Utilities|IsValid _returnvalue
            (:Is%20Valid
              (Utilities|Array|AddUnique (Variables|Default|GetSpawnedUnits) _returnvalue)
              (bind (_outhit _returnvalue_2) (Collision|LineTraceByChannel (Transformation|GetActorLocation _returnvalue) (- (Transformation|GetActorLocation _returnvalue) "0.000000,0.000000,2000.000000") "TraceTypeQuery1" false (Utilities|Array|MakeArray _returnvalue) "None"))
              (if _returnvalue_2
                (Transformation|SetActorLocation (.Location (Collision|BreakHitResult _outhit)) false false)))
            (:Is%20Not%20Valid
              _)))))
    (else
      (for _array_element_2 (Variables|Default|GetSpawnedUnits)
        (Actor|DestroyActor _array_element_2))
      (Variables|Default|SetSpawnedUnits (Utilities|Array|MakeArray))))
  (Utilities|FlowControl|Delay (Variables|Default|GetSpawnDelay))
  (CallFunction|SpawnCheck))

(fn ConstructionScript
  (bind _shutoffzone (Variables|Default|GetShutoffZone))
  (Components|Box|SetBoxExtent (Variables|Default|GetSpawnZone) (Variables|Default|GetSpawnZoneSize) true)
  (Components|Box|SetBoxExtent _shutoffzone (Variables|Default|GetShutOffZoneSize) true)
  (Transformation|SetRelativeLocation _shutoffzone (Variables|Default|GetShutOffZoneLocation) false false))