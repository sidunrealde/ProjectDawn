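; Base enemy character for humans, monsters and animals that patrols, chases and melee-attacks the hero, or flees.
; An AI state switch drives AIMoveTo loops for random or path patrols, chasing and fleeing, triggered by pawn sensing or damage.
; Attack montage notifies fire sphere-trace damage, and a polling distance check ends combat.
; It also handles looping elemental damage-over-time timers, and death grants XP, objective progress and loot.
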(event OnSeePawn(PawnSensing)
  (params (Pawn :type Pawn%20Object%20Reference))
  (bind _self self)
  ;[1 1 1] EnemyPerception
  (if (not (Variables|Booleans|GetIsDead))
    (if (Variables|Booleans|GetIsPassive)
      (if (Variables|Booleans|GetIsTimid)
        (Variables|Default|SetAIStates "NewEnumerator4")
        (Variables|Booleans|SetIsScared true)
        (CallFunction|BehaviourUnit))
      (else
        (bind _asbp_hero_base (Utilities|Casting|CastToBP_HeroBase Pawn))
        (Variables|Default|SetPlayerRef _asbp_hero_base)
        (Utilities|FlowControl|DoOnce false
          (:Completed
            (Utilities|Array|AddUnique (Variables|/Game/ProjectDawn/Blueprints/BP_HeroBase.BP_HeroBase_C|GetEnemyList (Variables|Default|GetPlayerRef)) _self)
            (bind _returnvalue (UserInterface|CreateWidget "/Game/ProjectDawn/Blueprints/HUD/W_EnemyList.W_EnemyList_C" 0 _self))
            (bind _output_get (Variables|Default|SetHudWidgetRef _returnvalue))
            (UserInterface|SetWidget (Variables|Default|GetEnemyStats) _output_get)
            (Variables|Default|SetAttackTarget (Variables|Default|GetPlayerRef))
            (Variables|Default|SetAIStates "NewEnumerator1")
            (Variables|Default|SetCombatStates "NewEnumerator0")
            (CallFunction|BehaviourUnit)
            (CallFunction|DisengageCheck)))))))

(event OnComponentBeginOverlap(InteractRadius)
  (params (OverlappedComponent :type Primitive%20Component%20Object%20Reference) (OtherActor :type Actor%20Object%20Reference) (OtherComp :type Primitive%20Component%20Object%20Reference) (OtherBodyIndex :type Integer) (bFromSweep :type Boolean) (SweepResult :type Hit%20Result%20Structure%20%28by%20ref%29))
  ;[1 1 1] OnOverlap
)

(event OnComponentEndOverlap(InteractRadius)
  (params (OverlappedComponent :type Primitive%20Component%20Object%20Reference) (OtherActor :type Actor%20Object%20Reference) (OtherComp :type Primitive%20Component%20Object%20Reference) (OtherBodyIndex :type Integer))
  ;[1 1 1] OnOverlap
)

(event Custom|MoveToPatrolPoint
  (bind _patrol_path (Variables|PatrolPath|GetPatrol%20Path))
  ;[1 1 1] EnemyBase Behaviour
  ;;[1 1 1] Move to PatrolPoint
  (if (Utilities|Enum|Equal(Enum) (Variables|Default|GetAIStates) "NewEnumerator1")
    (Variables|Default|SetCombatStates "NewEnumerator0")
    (bind _animation_duration (CallFunction|WeaponCheck))
    (Utilities|Time|SetTimerbyEvent (delegate Custom|StartChase) _animation_duration)
    (else
      (bind _keys (Utilities|Map|Keys (Variables|PatrolPath|GetPatrol%20Path)))
      (AI|AIMoveTo self (Transformation|GetActorLocation (Utilities|Array|Get(acopy) _keys (Variables|PatrolPath|GetCurrentPatrolIndex))) 0 5.0 false
        (:OnSuccess
          (bind _keys_2 (Utilities|Map|Keys _patrol_path))
          (Variables|PatrolPath|SetCurrentPatrolPoint (Utilities|Array|Get(acopy) _keys_2 (Variables|PatrolPath|GetCurrentPatrolIndex)))
          (Utilities|Time|SetTimerbyEvent (delegate Custom|OnEndWaiting) (Math|Float|Max(Float) (.Value (Utilities|Map|Find _patrol_path (Utilities|Array|Get(acopy) _keys_2 (Variables|PatrolPath|GetCurrentPatrolIndex)))) 0.1))
          (Default|OnPatrollerEntered (Utilities|Array|Get(acopy) _keys_2 (Variables|PatrolPath|GetCurrentPatrolIndex)) self))))))

(event Custom|OnEndWaiting
  ;[1 1 1] EnemyBase Behaviour
  ;;[1 1 1] Move to PatrolPoint
  (Default|OnPatrollerExit (Variables|PatrolPath|GetCurrentPatrolPoint))
  (bind _output_get (Variables|PatrolPath|SetCurrentPatrolIndex (+ (Variables|PatrolPath|GetCurrentPatrolIndex) (Variables|PatrolPath|GetReversePath))))
  (if (Utilities|Array|IsValidIndex (stale Custom|MoveToPatrolPoint _keys) _output_get)
    (CallFunction|MovetoPatrolPoint)
    (else
      (switch Utilities|FlowControl|Switch|SwitchonEN_PatrolPaths (Variables|PatrolPath|GetPatrol%20Path%20Type)
        (:NewEnumerator0
          (Variables|PatrolPath|SetCurrentPatrolIndex 0)
          (CallFunction|MovetoPatrolPoint))
        (:NewEnumerator1
          (Variables|PatrolPath|SetReversePath (* (Variables|PatrolPath|GetReversePath) -1))
          (Variables|PatrolPath|SetCurrentPatrolIndex (+ (Variables|PatrolPath|GetCurrentPatrolIndex) (Variables|PatrolPath|GetReversePath)))
          (CallFunction|MovetoPatrolPoint))))))

(event Custom|Flee
  (bind _returnvalue (Transformation|GetActorLocation))
  (bind _returnvalue_2 (Game|GetPlayerCharacter 0))
  (bind _returnvalue_3 (Transformation|GetActorLocation _returnvalue_2))
  (bind _returnvalue_4 (Math|Rotator|FindLookatRotation _returnvalue _returnvalue_3))
  (bind _returnvalue_5 (Math|Vector|GetForwardVector _returnvalue_4))
  (bind _returnvalue_6 (* _returnvalue_5 -5e+02))
  (bind _returnvalue_7 (+ _returnvalue _returnvalue_6))
  (bind (_x _y) (Math|Vector|BreakVector _returnvalue_7))
  ;[1 1 1] EnemyBase Behaviour
  (Audio|PlaySoundatLocation (Variables|Sound|GetFleeingSound) (Transformation|GetActorLocation) "0, 0, 0" 1.0 1.0 0.0 0 0 0 0)
  (if (not (Variables|Booleans|GetIsDead))
    (Variables|/Script/Engine.CharacterMovementComponent|SetMaxWalkSpeed (Variables|Character|GetCharacterMovement) (Variables|Stats|GetCombatWalkSpeed))
    (AI|AIMoveTo self (.RandomLocation (AI|Navigation|GetRandomReachablePointinRadius (Math|Vector|MakeVector _x _y (.Z (Math|Vector|BreakVector _returnvalue))) 3e+02 0 0)) 0 5.0 false
      (:OnSuccess
        _)
      (:OnFail
        _))
    (CallFunction|Flee)))

(event Custom|OnDead
  (bind _mesh (Variables|Character|GetMesh))
  (bind _returnvalue (Components|SkeletalMesh|GetAnimInstance _mesh))
  ;[1 1 1] Deal Damage
  (Utilities|FlowControl|DoOnce false
    (:Completed
      (Variables|Booleans|SetIsDead true)
      (Variables|/Game/ProjectDawn/Blueprints/Items/BC_LootBox.BC_LootBox_C|SetIsDead (Variables|Default|GetBC_LootBox) true)
      (bind _playerref (Variables|Default|GetPlayerRef)
        (:then
          (Default|GainXP _playerref (Variables|Stats|GetXP))
          (Components|Movement|StopMovementImmediately (Variables|Character|GetCharacterMovement))
          (if (Class|AnimInstance|IsAnyMontagePlaying _returnvalue)
            (Animation|Montage|MontageStop _returnvalue 0.0 (Animation|Montage|GetCurrentActiveMontage _returnvalue)))
          (Variables|Booleans|SetIsAttacking false)
          (Audio|PlaySoundatLocation (Variables|Sound|GetDeathSound) (Transformation|GetActorLocation) "0, 0, 0" 1.0 1.0 0.0 0 0 0 0)
          (Variables|Default|SetAIStates "NewEnumerator2")
          (CallFunction|BehaviourUnit)
          (UserInterface|SetWidget (Variables|Default|GetEnemyStats) 0)
          (Collision|SetCollisionResponsetoChannel (Variables|Character|GetMesh) "ECC_Visibility" "ECR_Ignore")
          (Collision|SetCollisionResponsetoChannel (Variables|Character|GetMesh) "ECC_Pawn" "ECR_Ignore")
          (Default|CallOnObjectiveIDCalled (Variables|Default|GetPlayerRef) (Variables|Default|GetObjectiveID) 1)
          (Utilities|FlowControl|Delay 3e+01)
          (Actor|DestroyActor))
        (:else)))))

(event Custom|StartDamageOverTime
  (params (SpellType :type EN_SpellType%20Enum :default "NewEnumerator0") (ElementalType :type EN_ElementalTypes%20Enum :default "NewEnumerator0") (Potency :type Float%20%28double-precision%29))
  (switch Utilities|FlowControl|Switch|SwitchonEN_SpellType SpellType
    (:NewEnumerator0
      _)
    (:NewEnumerator2
      _))
  (switch Utilities|FlowControl|Switch|SwitchonEN_ElementalTypes ElementalType
    (:NewEnumerator1
      (bind _returnvalue (Utilities|Time|SetTimerbyEvent (delegate Custom|FireDamageOverTime) 1.0 true))
      (Variables|Timers|SetElementalEffectTimer _returnvalue))
    (:NewEnumerator2
      (bind _returnvalue_2 (Utilities|Time|SetTimerbyEvent (delegate Custom|FreezeDamageOverTime) 1.0 true))
      (Variables|Timers|SetElementalEffectTimer _returnvalue_2))
    (:NewEnumerator3
      (bind _returnvalue_3 (Utilities|Time|SetTimerbyEvent (delegate Custom|ShockDamageOverTime) 1.0 true))
      (Variables|Timers|SetElementalEffectTimer _returnvalue_3))))

(event Custom|FireDamageOverTime
  (bind _isdead (CallFunction|FireDOT (stale Custom|StartDamageOverTime Potency)))
  (if _isdead
    (CallFunction|OnDead)))

(event Custom|FreezeDamageOverTime
  (bind _isdead (CallFunction|FreezeDOT (stale Custom|StartDamageOverTime Potency)))
  (if _isdead
    (CallFunction|OnDead)))

(event Custom|ShockDamageOverTime
  (bind _isdead (CallFunction|ShockDOT (stale Custom|StartDamageOverTime Potency)))
  (if _isdead
    (CallFunction|OnDead)))

(event Custom|EndElemetalEffect
  (params (ElementalType :type EN_ElementalTypes%20Enum :default "NewEnumerator0") (Duration :type Float%20%28single-precision%29))
  (switch Utilities|FlowControl|Switch|SwitchonEN_ElementalTypes ElementalType
    (:NewEnumerator1
      (CallFunction|StatusParticleEffects (Variables|ParticleSystems|GetFireEffect)))
    (:NewEnumerator2
      (CallFunction|StatusParticleEffects (Variables|ParticleSystems|GetFreezeEffect)))
    (:NewEnumerator3
      (CallFunction|StatusParticleEffects (Variables|ParticleSystems|GetShockEffect))))
  (Utilities|FlowControl|Delay Duration)
  (Utilities|Time|ClearandInvalidateTimerbyHandle (Variables|Timers|GetElementalEffectTimer))
  (CallFunction|ClearElementalEffects))

(event Custom|StartChase
  (CallFunction|ChasePlayer))

(event Custom|BehaviourUnit
  (bind _returnvalue (Transformation|GetActorLocation))
  (bind _returnvalue_2 (Game|GetPlayerCharacter 0))
  (bind _aipatrolpathcomponent (Variables|Default|GetAIPatrolPathComponent))
  (bind _charactermovement (Variables|Character|GetCharacterMovement))
  (bind _returnvalue_3 (Transformation|GetActorLocation _returnvalue_2))
  (bind _patrolpath (Variables|/Game/ProjectDawn/Blueprints/NPC/Enemies/AIBehaviourComponentPatrolPath.AIBehaviourComponentPatrolPath_C|GetPatrolPath _aipatrolpathcomponent))
  (bind _returnvalue_4 (Math|Rotator|FindLookatRotation _returnvalue _returnvalue_3))
  (bind _returnvalue_5 (Math|Vector|GetForwardVector _returnvalue_4))
  (bind _returnvalue_6 (* _returnvalue_5 -5e+02))
  (bind _returnvalue_7 (+ _returnvalue _returnvalue_6))
  (bind (_x _y) (Math|Vector|BreakVector _returnvalue_7))
  ;[1 1 1] EnemyBase Behaviour
  (if (not (Variables|Booleans|GetIsDead))
    (switch Utilities|FlowControl|Switch|SwitchonEN_AIStates (Variables|Default|GetAIStates)
      (:NewEnumerator0
        ;;[1 1 1] Patrol
        (switch Utilities|FlowControl|Switch|SwitchonEN_PatrolType (Variables|Default|GetPatrolType)
          (:NewEnumerator0
            ;;;[1 1 1] RandomPatrol
            (AI|AIMoveTo self (.RandomLocation (AI|Navigation|GetRandomReachablePointinRadius (Transformation|GetActorLocation) (Variables|RandomPatrol|GetRoamRadius) 0 0)) 0 5.0 false
              (:OnSuccess
                _)
              (:OnFail
                _))
            (Utilities|FlowControl|Delay (Math|Random|RandomFloatinRange (Variables|RandomPatrol|GetMinWaitTime) (Variables|RandomPatrol|GetMaxWaitTime)))
            (if (Variables|Booleans|GetIsScared)
              (CallFunction|Flee :!label _label)
              (elif (Utilities|Enum|Equal(Enum) (Variables|Default|GetAIStates) "NewEnumerator1")
                (bind _animation_duration (CallFunction|WeaponCheck))
                (Utilities|Time|SetTimerbyEvent (delegate Custom|StartChase) _animation_duration)
                (else
                  (CallFunction|RandomPatrol)))))
          (:NewEnumerator1
            ;;;[1 1 1] Follow Patrol Path
            (Variables|PatrolPath|SetPatrol%20Path (Utilities|Map|MakeMap))
            (Variables|PatrolPath|SetPatrol%20Path%20Type (Variables|/Game/ProjectDawn/Blueprints/NPC/Enemies/AIBehaviourComponentPatrolPath.AIBehaviourComponentPatrolPath_C|GetPatrolPathType _aipatrolpathcomponent))
            (Utilities|IsValid _aipatrolpathcomponent
              (:Is%20Valid
                (if (> (Utilities|Map|Length _patrolpath) 0)
                  (if (Variables|Booleans|GetIsScared)
                    (goto _label)
                    (else
                      (Variables|PatrolPath|SetPatrol%20Path _patrolpath)
                      (CallFunction|MovetoPatrolPoint)))))))))
      (:NewEnumerator1
        ;;[1 1 1] Chase Target
        (if (not (Variables|Booleans|GetIsDead))
          (AI|AIMoveTo self "0, 0, 0" (Variables|Default|GetAttackTarget) (Variables|Combat|GetAttackDistance) false
            (:OnSuccess
              (Utilities|FlowControl|DoOnce false
                (:Completed
                  (Variables|Booleans|SetIsAttacking true)
                  (bind _notifyname (Animation|Montage|PlayMontage (Variables|Character|GetMesh) (.OutItem (Utilities|Array|Random (Variables|Animations|GetAttackMontages))))
                    (:then
                      (Components|Movement|StopMovementImmediately _charactermovement)
                      (Variables|/Script/Engine.CharacterMovementComponent|SetMaxWalkSpeed _charactermovement 0.0)
                      (CallFunction|TrackPlayer)
                      (Audio|PlaySoundatLocation (Variables|Sound|GetAttackSwingSound) (Transformation|GetActorLocation) "0, 0, 0" 1.0 1.0 0.0 0 0 0 0))
                    (:OnCompleted
                      (Utilities|FlowControl|Delay (Math|Random|RandomFloatinRange 0.2 0.8))
                      (Variables|/Script/Engine.CharacterMovementComponent|SetMaxWalkSpeed _charactermovement (Variables|Stats|GetCombatWalkSpeed))
                      (Variables|Booleans|SetIsAttacking false)
                      (if (not (Variables|Booleans|GetIsDead))
                        (CallFunction|ReleaseAttack)
                        (CallFunction|BehaviourUnit)))
                    (:OnNotifyBegin
                      (switch name _notifyname
                        (:AttackTrace
                          (Audio|PlaySoundatLocation (Variables|Sound|GetAttackGruntSound) (Transformation|GetActorLocation) "0, 0, 0" 1.0 1.0 0.0 0 0 0 0)
                          (CallFunction|AttackTrace)))))))))))
      (:NewEnumerator4
        (if (not (Variables|Booleans|GetIsDead))
          (Variables|/Script/Engine.CharacterMovementComponent|SetMaxWalkSpeed (Variables|Character|GetCharacterMovement) (Variables|Stats|GetCombatWalkSpeed))
          (AI|AIMoveTo self (.RandomLocation (AI|Navigation|GetRandomReachablePointinRadius (Math|Vector|MakeVector _x _y (.Z (Math|Vector|BreakVector _returnvalue))) 3e+02 0 0)) 0 5.0 false
            (:OnSuccess
              _)
            (:OnFail
              _))
          (CallFunction|Flee))))))

(event Custom|RandomPatrol
  ;[1 1 1] EnemyBase Behaviour
  ;;[1 1 1] Patrol
  ;;;[1 1 1] RandomPatrol
  (if (not (Variables|Booleans|GetIsDead))
    (AI|AIMoveTo self (.RandomLocation (AI|Navigation|GetRandomReachablePointinRadius (Transformation|GetActorLocation) (Variables|RandomPatrol|GetRoamRadius) 0 0)) 0 5.0 false
      (:OnSuccess
        _)
      (:OnFail
        _))
    (Utilities|FlowControl|Delay (Math|Random|RandomFloatinRange (Variables|RandomPatrol|GetMinWaitTime) (Variables|RandomPatrol|GetMaxWaitTime)))
    (if (Variables|Booleans|GetIsScared)
      (CallFunction|Flee)
      (elif (Utilities|Enum|Equal(Enum) (Variables|Default|GetAIStates) "NewEnumerator1")
        (bind _animation_duration (CallFunction|WeaponCheck))
        (Utilities|Time|SetTimerbyEvent (delegate Custom|StartChase) _animation_duration)
        (else
          (CallFunction|RandomPatrol))))))

(event Custom|ChasePlayer
  (bind _charactermovement (Variables|Character|GetCharacterMovement))
  ;[1 1 1] EnemyBase Behaviour
  ;;[1 1 1] Chase Target
  (if (not (Variables|Booleans|GetIsDead))
    (AI|AIMoveTo self "0, 0, 0" (Variables|Default|GetAttackTarget) (Variables|Combat|GetAttackDistance) false
      (:OnSuccess
        (Utilities|FlowControl|DoOnce false
          (:Completed
            (Variables|Booleans|SetIsAttacking true)
            (bind _notifyname (Animation|Montage|PlayMontage (Variables|Character|GetMesh) (.OutItem (Utilities|Array|Random (Variables|Animations|GetAttackMontages))))
              (:then
                (Components|Movement|StopMovementImmediately _charactermovement)
                (Variables|/Script/Engine.CharacterMovementComponent|SetMaxWalkSpeed _charactermovement 0.0)
                (CallFunction|TrackPlayer)
                (Audio|PlaySoundatLocation (Variables|Sound|GetAttackSwingSound) (Transformation|GetActorLocation) "0, 0, 0" 1.0 1.0 0.0 0 0 0 0))
              (:OnCompleted
                (Utilities|FlowControl|Delay (Math|Random|RandomFloatinRange 0.2 0.8))
                (Variables|/Script/Engine.CharacterMovementComponent|SetMaxWalkSpeed _charactermovement (Variables|Stats|GetCombatWalkSpeed))
                (Variables|Booleans|SetIsAttacking false)
                (if (not (Variables|Booleans|GetIsDead))
                  (CallFunction|ReleaseAttack)
                  (CallFunction|BehaviourUnit)))
              (:OnNotifyBegin
                (switch name _notifyname
                  (:AttackTrace
                    (Audio|PlaySoundatLocation (Variables|Sound|GetAttackGruntSound) (Transformation|GetActorLocation) "0, 0, 0" 1.0 1.0 0.0 0 0 0 0)
                    (CallFunction|AttackTrace)))))))))))

(event Custom|ReleaseAttack
  (bind _charactermovement (Variables|Character|GetCharacterMovement))
  ;[1 1 1] EnemyBase Behaviour
  ;;[1 1 1] Chase Target
  (Utilities|FlowControl|DoOnce false) ; enters at Reset
)

(event Custom|TrackPlayer
  ;[1 1 1] EnemyBase Behaviour
  ;;[1 1 1] Rotate to faceplayer
  (Variables|Default|GetAttackTarget
    (:then
      (if (Variables|Booleans|GetIsAttacking)
        (Transformation|SetActorRotation (Math|Rotator|MakeRotator 0.0 0.0 (.yaw (Math|Rotator|FindLookatRotation (Transformation|GetActorLocation) (Transformation|GetActorLocation (Variables|Default|GetAttackTarget))))))
        (Utilities|FlowControl|Delay 0.01)
        (CallFunction|TrackPlayer)))
    (:else)))

(event Custom|Damaged
  (bind _self self)
  ;[1 1 1] EnemyPerception
  (Utilities|FlowControl|DoOnce false
    (:Completed
      (bind _asbp_hero_base (Utilities|Casting|CastToBP_HeroBase (stale OnSeePawn(PawnSensing) Pawn)))
      (Variables|Default|SetPlayerRef _asbp_hero_base)
      (Utilities|FlowControl|DoOnce false
        (:Completed
          (Utilities|Array|AddUnique (Variables|/Game/ProjectDawn/Blueprints/BP_HeroBase.BP_HeroBase_C|GetEnemyList (Variables|Default|GetPlayerRef)) _self)
          (bind _returnvalue (UserInterface|CreateWidget "/Game/ProjectDawn/Blueprints/HUD/W_EnemyList.W_EnemyList_C" 0 _self))
          (bind _output_get (Variables|Default|SetHudWidgetRef _returnvalue))
          (UserInterface|SetWidget (Variables|Default|GetEnemyStats) _output_get)
          (Variables|Default|SetAttackTarget (Variables|Default|GetPlayerRef))
          (Variables|Default|SetAIStates "NewEnumerator1")
          (Variables|Default|SetCombatStates "NewEnumerator0")
          (CallFunction|BehaviourUnit)
          (CallFunction|DisengageCheck))))))

(event Custom|DisengageCheck
  (bind _disengagerange (Variables|Combat|GetDisengageRange))
  (bind _disengagerangestandarddeviation (Variables|Combat|GetDisengageRangeStandardDeviation))
  ;[1 1 1] Disengage combat
  (bind _playerref (Variables|Default|GetPlayerRef)
    (:then
      (if (>= (Transformation|GetDistanceTo _playerref) (.OutItem (Utilities|Array|Random (Utilities|Array|MakeArray (+ _disengagerange _disengagerangestandarddeviation) (- _disengagerange _disengagerangestandarddeviation)))))
        (Variables|Booleans|SetIsAttacking false)
        (Variables|Default|SetAIStates "NewEnumerator0")
        (bind _animationduration (CallFunction|ResetCombat))
        (Utilities|FlowControl|Delay _animationduration)
        (CallFunction|BehaviourUnit)
        (UserInterface|SetWidget (Variables|Default|GetEnemyStats) 0)
        (CallFunction|ResetDoOnce)
        (else
          (Utilities|FlowControl|Delay 1.0)
          (CallFunction|DisengageCheck))))
    (:else)))

(event Custom|ResetDoOnce
  (bind _self self)
  ;[1 1 1] EnemyPerception
  (Utilities|FlowControl|Sequence
    (:then_0
      (Utilities|FlowControl|DoOnce false) ; enters at Reset
    )
    (:then_1
      (Utilities|FlowControl|DoOnce false) ; enters at Reset
    )
    (:then_2
      (Utilities|FlowControl|DoOnce false) ; enters at Reset
    )))

(event EventOnEnemyArrowHit
  (bind _self self)
  ;[1 1 1] EnemyPerception
  (Utilities|FlowControl|DoOnce false
    (:Completed
      (bind _asbp_hero_base (Utilities|Casting|CastToBP_HeroBase (Game|GetPlayerCharacter 0)))
      (Variables|Default|SetPlayerRef _asbp_hero_base)
      (if (not (Variables|Booleans|GetIsTimid))
        (Utilities|FlowControl|DoOnce false
          (:Completed
            (Utilities|Array|AddUnique (Variables|/Game/ProjectDawn/Blueprints/BP_HeroBase.BP_HeroBase_C|GetEnemyList (Variables|Default|GetPlayerRef)) _self)
            (bind _returnvalue (UserInterface|CreateWidget "/Game/ProjectDawn/Blueprints/HUD/W_EnemyList.W_EnemyList_C" 0 _self))
            (bind _output_get (Variables|Default|SetHudWidgetRef _returnvalue))
            (UserInterface|SetWidget (Variables|Default|GetEnemyStats) _output_get)
            (Variables|Default|SetAttackTarget (Variables|Default|GetPlayerRef))
            (Variables|Default|SetAIStates "NewEnumerator1")
            (Variables|Default|SetCombatStates "NewEnumerator0")
            (CallFunction|BehaviourUnit)
            (CallFunction|DisengageCheck)))))))

(event EventInteract
  ;[1 1 1] Interact Loot
  (Default|LootMenu (Variables|Default|GetBC_LootBox)))

(event EventElementalEffect
  (params (Potency :type Float%20%28double-precision%29) (SpellType :type EN_SpellType%20Enum :default "NewEnumerator0") (ElementalType :type EN_ElementalTypes%20Enum :default "NewEnumerator0"))
  (CallFunction|StartDamageOverTime SpellType ElementalType Potency))

(event EventBeginPlay
  ;[1 1 1] BeginPlay
  (CallFunction|BehaviourUnit)
  (Variables|/Script/Engine.CharacterMovementComponent|SetMaxWalkSpeed (Variables|Character|GetCharacterMovement) (Variables|Stats|GetPatrolWalkSpeed))
  (Variables|/Game/ProjectDawn/Blueprints/Items/BC_LootBox.BC_LootBox_C|SetLootName (Variables|Default|GetBC_LootBox) (Variables|Stats|GetEnemyName)))

(event EventTimerEndEffect
  (params (Duration :type Float%20%28double-precision%29) (ElementType :type EN_ElementalTypes%20Enum :default "NewEnumerator0"))
  (CallFunction|EndElemetalEffect ElementType Duration))

(event Game|Damage|EventAnyDamage
  (params (Damage :type Float%20%28single-precision%29) (DamageType :type Damage%20Type%20Object%20Reference) (InstigatedBy :type Controller%20Object%20Reference) (DamageCauser :type Actor%20Object%20Reference))
  (bind _mesh (Variables|Character|GetMesh))
  (bind _returnvalue (Components|SkeletalMesh|GetAnimInstance _mesh))
  ;[1 1 1] Deal Damage
  (bind _asbp_hero_base (Utilities|Casting|CastToBP_HeroBase DamageCauser))
  (Variables|Default|SetPlayerRef _asbp_hero_base)
  (bind _output_get (Variables|Stats|SetHealth (- (Variables|Stats|GetHealth) Damage)))
  (if (<= _output_get 0.0)
    (Utilities|FlowControl|DoOnce false
      (:Completed
        (Variables|Booleans|SetIsDead true)
        (Variables|/Game/ProjectDawn/Blueprints/Items/BC_LootBox.BC_LootBox_C|SetIsDead (Variables|Default|GetBC_LootBox) true)
        (bind _playerref (Variables|Default|GetPlayerRef)
          (:then
            (Default|GainXP _playerref (Variables|Stats|GetXP))
            (Components|Movement|StopMovementImmediately (Variables|Character|GetCharacterMovement))
            (if (Class|AnimInstance|IsAnyMontagePlaying _returnvalue)
              (Animation|Montage|MontageStop _returnvalue 0.0 (Animation|Montage|GetCurrentActiveMontage _returnvalue)))
            (Variables|Booleans|SetIsAttacking false)
            (Audio|PlaySoundatLocation (Variables|Sound|GetDeathSound) (Transformation|GetActorLocation) "0, 0, 0" 1.0 1.0 0.0 0 0 0 0)
            (Variables|Default|SetAIStates "NewEnumerator2")
            (CallFunction|BehaviourUnit)
            (UserInterface|SetWidget (Variables|Default|GetEnemyStats) 0)
            (Collision|SetCollisionResponsetoChannel (Variables|Character|GetMesh) "ECC_Visibility" "ECR_Ignore")
            (Collision|SetCollisionResponsetoChannel (Variables|Character|GetMesh) "ECC_Pawn" "ECR_Ignore")
            (Default|CallOnObjectiveIDCalled (Variables|Default|GetPlayerRef) (Variables|Default|GetObjectiveID) 1)
            (Utilities|FlowControl|Delay 3e+01)
            (Actor|DestroyActor))
          (:else))))
    (else
      (CallFunction|Damaged))))

(fn ConstructionScript)

(fn WeaponCheck
  (if (not (Variables|Booleans|GetIsDead))
    (Variables|/Script/Engine.CharacterMovementComponent|SetMaxWalkSpeed (Variables|Character|GetCharacterMovement) (Variables|Stats|GetCombatWalkSpeed))
    (switch Utilities|FlowControl|Switch|SwitchonEN_EnemyType (Variables|Combat|GetEnemyType)
      (:NewEnumerator0
        (switch Utilities|FlowControl|Switch|SwitchonEN_CombatStates (Variables|Default|GetCombatStates)
          (:NewEnumerator0
            (Variables|Booleans|SetIsMeleeCombat true)
            (if (Variables|Booleans|GetIsRangedCombat)
              (bind _returnvalue (Animation|PlayAnimMontage (Variables|Animations|GetStowRangedWeaponMontage) (Variables|Animations|GetStowRangedWeaponWeaponMontagePlayRate) "None"))
              (bind _returnvalue_2 (Animation|PlayAnimMontage (Variables|Animations|GetDrawMeleeWeaponMontage) (Variables|Animations|GetDraw%20Melee%20Weapon%20Montage%20Play%20Rate) "None"))
              (Variables|Booleans|SetIsRangedCombat false)
              (return (+ _returnvalue _returnvalue_2))
              (else
                (bind _returnvalue_3 (Animation|PlayAnimMontage (Variables|Animations|GetDrawMeleeWeaponMontage) (Variables|Animations|GetDraw%20Melee%20Weapon%20Montage%20Play%20Rate) "None"))
                ;[1 1 1] Temp
                (Audio|PlaySoundatLocation (Variables|Sound|GetEnemyAggroSound) (Transformation|GetActorLocation) "0, 0, 0" 1.0 1.0 0.0 0 0 0 0)
                (return _returnvalue_3))))
          (:NewEnumerator1
            (Variables|Booleans|SetIsRangedCombat true)
            (if (Variables|Booleans|GetIsMeleeCombat)
              (bind _returnvalue_4 (Animation|PlayAnimMontage (Variables|Animations|GetStowMeleeWeaponMontage) (Variables|Animations|GetStowMeleeWeaponMontageplayRate) "None"))
              (bind _returnvalue_5 (Animation|PlayAnimMontage (Variables|Animations|GetDrawRangedWeaponMontage) (Variables|Animations|GetDrawRangedWeaponMontagePlayRate) "None"))
              (Variables|Booleans|SetIsMeleeCombat false)
              (return (+ _returnvalue_5 _returnvalue_4))
              (else
                (bind _returnvalue_6 (Animation|PlayAnimMontage (Variables|Animations|GetDrawRangedWeaponMontage) (Variables|Animations|GetDrawRangedWeaponMontagePlayRate) "None"))
                (return _returnvalue_6))))))
      (:NewEnumerator1
        _)
      (:NewEnumerator2
        _))
    (Components|Movement|StopMovementImmediately (Variables|Character|GetCharacterMovement))
    (bind _returnvalue_7 (Animation|PlayAnimMontage (Variables|Animations|GetEnemy%20Aggro%20Animation%20Montage) (Variables|Animations|GetEnemyAggroAnimationPlayRate) "None"))
    ;[1 1 1] Temp
    (Audio|PlaySoundatLocation (Variables|Sound|GetEnemyAggroSound) (Transformation|GetActorLocation) "0, 0, 0" 1.0 1.0 0.0 0 0 0 0)
    (return _returnvalue_7)))

(fn ResetCombat
  (bind _charactermovement (Variables|Character|GetCharacterMovement))
  (switch Utilities|FlowControl|Switch|SwitchonEN_EnemyType (Variables|Combat|GetEnemyType)
    (:NewEnumerator0
      (switch Utilities|FlowControl|Switch|SwitchonEN_CombatStates (Variables|Default|GetCombatStates)
        (:NewEnumerator0
          (bind _returnvalue (Animation|PlayAnimMontage (Variables|Animations|GetStowMeleeWeaponMontage) 1.0 "None"))
          (Variables|Booleans|SetIsMeleeCombat false)
          (Variables|/Script/Engine.CharacterMovementComponent|SetMaxWalkSpeed _charactermovement (Variables|Stats|GetPatrolWalkSpeed))
          (Variables|Default|SetCombatStates "NewEnumerator2")
          (return _returnvalue))
        (:NewEnumerator1
          (bind _returnvalue_2 (Animation|PlayAnimMontage (Variables|Animations|GetStowRangedWeaponMontage) 1.0 "None"))
          (Variables|Booleans|SetIsRangedCombat false)
          (Variables|/Script/Engine.CharacterMovementComponent|SetMaxWalkSpeed _charactermovement (Variables|Stats|GetPatrolWalkSpeed))
          (Variables|Default|SetCombatStates "NewEnumerator2")
          (return _returnvalue_2))))
    (:NewEnumerator1
      _)
    (:NewEnumerator2
      _))
  (Variables|Booleans|SetIsMeleeCombat false)
  (Variables|Default|SetCombatStates "NewEnumerator2")
  (Variables|/Script/Engine.CharacterMovementComponent|SetMaxWalkSpeed (Variables|Character|GetCharacterMovement) (Variables|Stats|GetPatrolWalkSpeed))
  (return 0.0))

(fn AttackTrace
  (bind _returnvalue (Transformation|GetActorLocation))
  (bind _attackdamage (Variables|Stats|GetAttackDamage))
  (bind _attackdamagedeviation (Variables|Combat|GetAttackDamageDeviation))
  (bind (_outhit _returnvalue_2) (Collision|SphereTraceByChannel _returnvalue (+ _returnvalue (* (Transformation|GetActorForwardVector) (Variables|Combat|GetAttackRange))) (Variables|Combat|GetAttackTraceRadius) "TraceTypeQuery3" false 0 "None"))
  (if _returnvalue_2
    (Game|Damage|ApplyDamage (.HitActor (Collision|BreakHitResult _outhit)) (Math|Conversions|ToFloat(Integer) (Math|Float|Round (Math|Random|RandomFloatinRange (- _attackdamage _attackdamagedeviation) (+ _attackdamage _attackdamagedeviation)))) 0 0)
    (Audio|PlaySoundatLocation (Variables|Sound|GetAttackHitSound) (.Location (Collision|BreakHitResult _outhit)) "0, 0, 0" 1.0 1.0 0.0 0 0 0 0)))

(fn TakeAllLoot
  (for _array_element "NewEnumerator0"
    (bind _returnvalue (Utilities|GetDataTableRow "/Game/ProjectDawn/Blueprints/Items/Data/DT_ItemInfo.DT_ItemInfo" (Utilities|String|StringToName (Utilities|String|EnumtoString _array_element)))
      (:then
        (Default|PickupItem (Variables|Default|GetPlayerRef) _returnvalue)))))

(fn FireDOT
  (params (Potency :type Float%20%28double-precision%29))
  (bind _output_get (Variables|Stats|SetHealth (- (Variables|Stats|GetHealth) Potency)))
  (return (<= _output_get 0.0)))

(fn FreezeDOT
  (params (Potency :type Float%20%28double-precision%29))
  (Variables|/Script/Engine.CharacterMovementComponent|SetMaxWalkSpeed (Variables|Character|GetCharacterMovement) 1.5e+02)
  (bind _output_get (Variables|Stats|SetHealth (- Potency (Variables|Stats|GetHealth))))
  (return (<= _output_get 0.0)))

(fn ShockDOT
  (params (Potency :type Float%20%28double-precision%29))
  (Variables|/Script/Engine.CharacterMovementComponent|SetMaxWalkSpeed (Variables|Character|GetCharacterMovement) 2e+02)
  (bind _output_get (Variables|Stats|SetHealth (- 0.0 (Variables|Stats|GetHealth))))
  (return (<= _output_get 0.0)))

(fn StatusParticleEffects
  (params (EmitterTemplate :type Particle%20System%20Object%20Reference))
  (bind _returnvalue (Effects|SpawnEmitterAttached EmitterTemplate (Variables|Character|GetMesh) "None" "0, 0, 0" "0, 0, 0" "1.000000,1.000000,1.000000" "SnapToTargetIncludingScale"))
  (Variables|Default|SetActiveElementalParticleSystem _returnvalue))

(fn ClearElementalEffects
  (Variables|/Script/Engine.CharacterMovementComponent|SetMaxWalkSpeed (Variables|Character|GetCharacterMovement) (Variables|Stats|GetCombatWalkSpeed))
  (Utilities|IsValid (Variables|Default|GetActiveElementalParticleSystem)
    (:Is%20Valid
      (Components|DestroyComponent (Variables|Default|GetActiveElementalParticleSystem))
      (Variables|Default|SetActiveElementalParticleSystem 0))))

(fn EnemyRef
  (return self))

(fn QuestInteract
  (return ""))