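; Shopkeeper NPC Blueprint that links a dialogue component to a shop component for Shop001.
; QuestInteract readies the dialogue camera, opens the conversation, sets IsTalking and returns the BCShopKeeper component's interact result.
; The dialogue component's shopkeeper-widget event, bound on BeginPlay, opens the shop and passes this NPC to the shop widget.
; Closing either the conversation or the shop clears IsTalking.
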(event Custom|ConversationClosed
  (Variables|Default|SetIsTalking false))

(event Custom|QuestWidgetDisplay
  (bind _bc_shopkeeper (Variables|Default|GetBC_ShopKeeper))
  (bind _shopwidgetref (Variables|/Game/ProjectDawn/Blueprints/NPC/ShopKeeperNpc/BC_ShopKeeper.BC_ShopKeeper_C|GetShopWidgetRef _bc_shopkeeper))
  (Default|OpenShop (Variables|Default|GetBC_ShopKeeper))
  (Utilities|IsValid _shopwidgetref
    (:Is%20Valid
      (Variables|/Game/ProjectDawn/Blueprints/HUD/Shop/W_Shop.W_Shop_C|SetShopKeeperRef _shopwidgetref self)
      (EventDispatchers|BindEventtoOnShopClosed _shopwidgetref (delegate Custom|QuestAcceptEvent)))))

(event Custom|QuestAcceptEvent
  (Variables|Default|SetIsTalking false))

(event EventBeginPlay
  (|CallParentFunction)
  (Utilities|FlowControl|Sequence
    (:then_0
      (Variables|/Game/ProjectDawn/Blueprints/Dialogue/BC_DialogueBaseComponent.BC_DialogueBaseComponent_C|SetNPCRef (Variables|Default|GetBCC_DialogueShopNPC_01) self)
      (EventDispatchers|BindEventtoOnShopkeeperWidget (Variables|Default|GetBCC_DialogueShopNPC_01) (delegate Custom|QuestWidgetDisplay)))
    (:then_1
      (EventDispatchers|BindEventtoOnConversationClosed (Variables|Default|GetBCC_DialogueShopNPC_01) (delegate Custom|ConversationClosed)))))

(event Collision|EventActorBeginOverlap
  (params (OtherActor :type Actor%20Object%20Reference))
  (|CallParentFunction OtherActor) ; This node is disabled and will not be called.\nDrag off pins to build functionality.
)

(event EventTick
  (params (DeltaSeconds :type Float%20%28single-precision%29))
  (|CallParentFunction DeltaSeconds) ; This node is disabled and will not be called.\nDrag off pins to build functionality.
)

(fn ConstructionScript
  (|CallParentFunction))

(fn QuestInteract
  (CallFunction|ReadyDialoguePlayerCamera)
  (Default|OpenConversation (Variables|Default|GetBCC_DialogueShopNPC_01))
  (Variables|Default|SetIsTalking true)
  (bind _objectiveid (Default|QuestInteract (Variables|Default|GetBC_ShopKeeper)))
  (return _objectiveid))