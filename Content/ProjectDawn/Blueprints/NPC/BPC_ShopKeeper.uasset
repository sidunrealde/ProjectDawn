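; Shopkeeper NPC actor that opens and closes a shop UI on interaction, with mesh and animation chosen in the construction script.
; Opening resolves expected inventory entries through DT_ItemInfo, blends the camera to the shopkeeper and shows W_Shop with mouse input.
; Closing restores game input and the player camera, and also triggers when the player leaves the sphere.
; The open state is mirrored on the player's BP_HeroBase.
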(event OnComponentEndOverlap(Sphere)
  (params (OverlappedComponent :type Primitive%20Component%20Object%20Reference) (OtherActor :type Actor%20Object%20Reference) (OtherComp :type Primitive%20Component%20Object%20Reference) (OtherBodyIndex :type Integer))
  (if (and (Variables|Default|GetIsShopOpen) (Actor|ActorHasTag OtherActor "Player"))
    (CallFunction|CheckifShopNeedstoClose)))

(event Custom|ShowShop
  (bind _returnvalue (Game|GetPlayerController 0))
  ;[1 1 1] ShowShopEvent
  (bind _returnvalue_2 (UserInterface|CreateWidget "/Game/ProjectDawn/Blueprints/HUD/Shop/W_Shop.W_Shop_C"))
  (Variables|/Game/ProjectDawn/Blueprints/HUD/Shop/W_Shop.W_Shop_C|SetShopKeeper _returnvalue_2 self)
  (bind _output_get (Variables|Default|SetShopWidgetRef _returnvalue_2))
  (UserInterface|Viewport|AddtoViewport _output_get 0)
  (Input|SetInputModeGameandUI _returnvalue _output_get "DoNotLock" true false)
  (Variables|/Script/Engine.PlayerController|SetbShowMouseCursor _returnvalue true)
  (Variables|Default|SetIsShopOpen true))

(event Custom|CheckIfShopNeedsToClose
  (bind _returnvalue (Game|GetPlayerController 0))
  (bind _inventoryexpected (Variables|Default|GetInventoryExpected))
  (if (Variables|Default|GetIsShopOpen)
    ;[1 1 1] CloseShop
    (Widget|RemovefromParent (Variables|Default|GetShopWidgetRef))
    (Input|SetInputModeGameOnly _returnvalue false)
    (Variables|/Script/Engine.PlayerController|SetbShowMouseCursor _returnvalue false)
    (Variables|Default|SetIsShopOpen false)
    (Game|Player|SetViewTargetwithBlend (Game|GetPlayerController 0) (Game|Player|GetPlayerPawn 0) 0.5 "VTBlend_Linear" 0.0 false)
    (Variables|/Game/ProjectDawn/Blueprints/BP_HeroBase.BP_HeroBase_C|SetIsShopOpen (Variables|Default|GetPlayerRef) false)
    (else
      ;[1 1 1] OpenShop
      (for _index (range 0 (- (Utilities|Array|Length _inventoryexpected) 1))
        (bind _returnvalue_2 (Utilities|GetDataTableRow "/Game/ProjectDawn/Blueprints/Items/Data/DT_ItemInfo.DT_ItemInfo" (Utilities|String|StringToName (Utilities|String|EnumtoString (Utilities|Array|Get(acopy) _inventoryexpected _index))))
          (:then
            (Utilities|Array|AddUnique (Variables|Default|GetInventory) _returnvalue_2)
            (Game|Player|SetViewTargetwithBlend (Game|GetPlayerController 0) self 0.5 "VTBlend_Linear" 0.0 false))))
      (CallFunction|ShowShop)
      (Variables|/Game/ProjectDawn/Blueprints/BP_HeroBase.BP_HeroBase_C|SetIsShopOpen (Variables|Default|GetPlayerRef) true))))

(event EventBeginPlay
  (bind _asbp_hero_base (Utilities|Casting|CastToBP_HeroBase (Game|GetPlayerCharacter 0)))
  (Variables|Default|SetPlayerRef _asbp_hero_base))

(event EventInteract
  (bind _returnvalue (Game|GetPlayerController 0))
  (bind _inventoryexpected (Variables|Default|GetInventoryExpected))
  (if (Variables|Default|GetIsShopOpen)
    ;[1 1 1] CloseShop
    (Widget|RemovefromParent (Variables|Default|GetShopWidgetRef))
    (Input|SetInputModeGameOnly _returnvalue false)
    (Variables|/Script/Engine.PlayerController|SetbShowMouseCursor _returnvalue false)
    (Variables|Default|SetIsShopOpen false)
    (Game|Player|SetViewTargetwithBlend (Game|GetPlayerController 0) (Game|Player|GetPlayerPawn 0) 0.5 "VTBlend_Linear" 0.0 false)
    (Variables|/Game/ProjectDawn/Blueprints/BP_HeroBase.BP_HeroBase_C|SetIsShopOpen (Variables|Default|GetPlayerRef) false)
    (else
      ;[1 1 1] OpenShop
      (for _index (range 0 (- (Utilities|Array|Length _inventoryexpected) 1))
        (bind _returnvalue_2 (Utilities|GetDataTableRow "/Game/ProjectDawn/Blueprints/Items/Data/DT_ItemInfo.DT_ItemInfo" (Utilities|String|StringToName (Utilities|String|EnumtoString (Utilities|Array|Get(acopy) _inventoryexpected _index))))
          (:then
            (Utilities|Array|AddUnique (Variables|Default|GetInventory) _returnvalue_2)
            (Game|Player|SetViewTargetwithBlend (Game|GetPlayerController 0) self 0.5 "VTBlend_Linear" 0.0 false))))
      (CallFunction|ShowShop)
      (Variables|/Game/ProjectDawn/Blueprints/BP_HeroBase.BP_HeroBase_C|SetIsShopOpen (Variables|Default|GetPlayerRef) true))))

(fn ConstructionScript
  (bind _shopkeep (Variables|Default|GetShopkeep))
  (|CallParentFunction)
  (Components|SkeletalMesh|SetSkeletalMeshAsset _shopkeep (Variables|Default|GetPickSkeletalMesh))
  (Components|Animation|OverrideAnimationData _shopkeep (Utilities|Select :Index (Variables|Default|GetNPCList) :NewEnumerator0 "/Game/ProjectDawn/Characters/NPC/ShopKeeps/001_Ichigo/Animations/Ichigo_talking.Ichigo_talking" :NewEnumerator1 "/Game/ProjectDawn/Characters/NPC/MagicTeachers/002_Midnight/Animations/MidnightIdle.MidnightIdle" :NewEnumerator5 0 :NewEnumerator6 0 :NewEnumerator7 0 :NewEnumerator8 0 :NewEnumerator9 "/Game/ProjectDawn/Characters/NPC/MagicTeachers/001_Angelica/Anims/AngelicaIdle.AngelicaIdle" :NewEnumerator10 "/Game/ProjectDawn/Characters/NPC/Quest/003_Kanato/Animations/Kanato_Idle.Kanato_Idle") true true 0.0 1.0))