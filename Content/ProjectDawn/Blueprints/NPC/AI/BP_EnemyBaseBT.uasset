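; Base enemy character Blueprint that supplies combat actions and settings, apparently for a behavior tree, such as enemy type, patrol type and melee range.
; WeaponCheck sets combat flags, then plays draw or stow montages for melee or ranged humans, or an aggro montage for monsters and animals.
; ResetCombat clears those flags, stows human weapons and resets the WeaponCheckDone blackboard key.
; MeleeAttack plays a random attack montage, and BeginPlay applies the walk speed.
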(event EventBeginPlay
  (Variables|/Script/Engine.CharacterMovementComponent|SetMaxWalkSpeed (Variables|Character|GetCharacterMovement) (Variables|Stats|GetMax%20Walk%20Speed)))

(fn ConstructionScript)

(fn EnemyTypeSelect
  (return (Variables|Type|GetSelectEnemyType)))

(fn MeleeAttack
  (bind _returnvalue (Animation|PlayAnimMontage (.OutItem (Utilities|Array|Random (Variables|AnimationMontages|GetMeleeAttackAnimationMontage))) 1.0 "None"))
  (return _returnvalue))

(fn MeleeAttackRange
  (return (Variables|Stats|GetMeleeDistance)))

(fn PatroltypeSelect
  (return (Variables|Type|GetPatrolType)))

(fn ResetCombat
  ;[1 1 1] Reset to Patrol
  (switch Utilities|FlowControl|Switch|SwitchonEN_EnemyType (Variables|Type|GetSelectEnemyType)
    (:NewEnumerator0
      (switch Utilities|FlowControl|Switch|SwitchonEN_CombatStates "NewEnumerator0"
        (:NewEnumerator0
          (bind _returnvalue (Animation|PlayAnimMontage (Variables|AnimationMontages|GetStowMeleeWeaponMontage) 1.0 "None"))
          (Variables|Booleans|SetMeleeCombat false)
          (AI|Components|Blackboard|SetValueasBool (AI|GetBlackboard 0) (Utilities|Name|MakeLiteralName "WeaponCheckDone") false)
          (return _returnvalue))
        (:NewEnumerator1
          (bind _returnvalue_2 (Animation|PlayAnimMontage (Variables|AnimationMontages|GetStowRangedWeaponMontage) 1.0 "None"))
          (Variables|Booleans|SetRangedCombat false)
          (AI|Components|Blackboard|SetValueasBool (AI|GetBlackboard 0) (Utilities|Name|MakeLiteralName "WeaponCheckDone") false)
          (return _returnvalue_2))))
    (:NewEnumerator1
      _)
    (:NewEnumerator2
      _))
  (Variables|Booleans|SetMeleeCombat false)
  (AI|Components|Blackboard|SetValueasBool (AI|GetBlackboard 0) (Utilities|Name|MakeLiteralName "WeaponCheckDone") false)
  (return 0.0))

(fn WeaponCheck
  (switch Utilities|FlowControl|Switch|SwitchonEN_EnemyType (Variables|Type|GetSelectEnemyType)
    (:NewEnumerator0
      (switch Utilities|FlowControl|Switch|SwitchonEN_CombatStates "NewEnumerator0"
        (:NewEnumerator0
          (Variables|Booleans|SetMeleeCombat true)
          (if (Variables|Booleans|GetRangedCombat)
            (bind _returnvalue (Animation|PlayAnimMontage (Variables|AnimationMontages|GetStowRangedWeaponMontage) (Variables|AnimationMontages|GetStowRangedWeaponWeaponMontagePlayRate) "None"))
            (return _returnvalue)
            (else
              (bind _returnvalue_2 (Animation|PlayAnimMontage (Variables|AnimationMontages|GetDrawMeleeWeaponMontage) (Variables|AnimationMontages|GetDrawMeleeWeaponMontagePlayRate) "None"))
              (return _returnvalue_2))))
        (:NewEnumerator1
          (Variables|Booleans|SetRangedCombat true)
          (if (Variables|Booleans|GetMeleeCombat)
            (bind _returnvalue_3 (Animation|PlayAnimMontage (Variables|AnimationMontages|GetStowMeleeWeaponMontage) (Variables|AnimationMontages|GetStowMeleeWeaponMontageplayRate) "None"))
            (return _returnvalue_3)
            (else
              (bind _returnvalue_4 (Animation|PlayAnimMontage (Variables|AnimationMontages|GetDrawRangedWeaponMontage) (Variables|AnimationMontages|GetDrawRangedWeaponMontagePlayRate) "None"))
              (return _returnvalue_4))))))
    (:NewEnumerator1
      _)
    (:NewEnumerator2
      _))
  (Variables|Booleans|SetMeleeCombat true)
  (bind _returnvalue_5 (Animation|PlayAnimMontage (Variables|AnimationMontages|GetEnemy%20Aggro%20Animation%20Montage) (Variables|AnimationMontages|GetEnemyAggroAnimationPlayRate) "None"))
  (return _returnvalue_5))