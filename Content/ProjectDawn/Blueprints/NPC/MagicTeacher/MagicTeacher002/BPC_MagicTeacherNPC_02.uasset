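; BPC_MagicTeacherNPC_02 is a magic teacher NPC that talks with the player and opens a magic shop.
; QuestInteract readies the dialogue camera, opens the conversation, sets IsTalking and returns the teacher component's QuestInteract result.
; The dialogue component's shopkeeper event opens the shop through BCMagicTeacherComponent and links its widget back to the NPC.
; Closing the conversation or the shop clears IsTalking.
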(event Custom|ConversationClosed
  (Variables|Default|SetIsTalking false))

(event Custom|QuestWidgetDisplay
  (bind _bc_magicteachercomponent (Variables|Default|GetBC_MagicTeacherComponent))
  (bind _shopwidgetref (Variables|/Game/ProjectDawn/Blueprints/NPC/MagicTeacher/BC_MagicTeacherComponent.BC_MagicTeacherComponent_C|GetShopWidgetRef _bc_magicteachercomponent))
  (Default|OpenShop _bc_magicteachercomponent)
  (Utilities|IsValid _shopwidgetref
    (:Is%20Valid
      (Variables|/Game/ProjectDawn/Blueprints/HUD/MagicShop/W_MagicShop.W_MagicShop_C|SetMagicTeacherRef _shopwidgetref self)
      (EventDispatchers|BindEventtoOnMagicShopClosed _shopwidgetref (delegate Custom|QuestAcceptEvent)))))

(event Custom|QuestAcceptEvent
  (Variables|Default|SetIsTalking false))

(event EventBeginPlay
  (bind _bcc_dialoguemagicteachernpc_02 (Variables|Default|GetBCC_DialogueMagicTeacherNPC_02))
  (|CallParentFunction)
  (Utilities|FlowControl|Sequence
    (:then_0
      (Variables|/Game/ProjectDawn/Blueprints/Dialogue/BC_DialogueBaseComponent.BC_DialogueBaseComponent_C|SetNPCRef _bcc_dialoguemagicteachernpc_02 self)
      (EventDispatchers|BindEventtoOnShopkeeperWidget _bcc_dialoguemagicteachernpc_02 (delegate Custom|QuestWidgetDisplay)))
    (:then_1
      (EventDispatchers|BindEventtoOnConversationClosed (Variables|Default|GetBCC_DialogueMagicTeacherNPC_02) (delegate Custom|ConversationClosed)))))

(event Collision|EventActorBeginOverlap
  (params (OtherActor :type Actor%20Object%20Reference))
  (|CallParentFunction OtherActor) ; This node is disabled and will not be called.\nDrag off pins to build functionality.
)

(event EventTick
  (params (DeltaSeconds :type Float%20%28single-precision%29))
  (|CallParentFunction DeltaSeconds) ; This node is disabled and will not be called.\nDrag off pins to build functionality.
)

(fn ConstructionScript
  (|CallParentFunction))

(fn QuestInteract
  (CallFunction|ReadyDialoguePlayerCamera)
  (Default|OpenConversation (Variables|Default|GetBCC_DialogueMagicTeacherNPC_02))
  (Variables|Default|SetIsTalking true)
  (bind _objectiveid (Default|QuestInteract (Variables|Default|GetBC_MagicTeacherComponent)))
  (return _objectiveid))