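; Magic teacher NPC actor that opens a spell shop when the player interacts with it.
; Interact toggles the shop: opening fills SpellInventory from the DT_Spells rows of its expected spells, blends the camera to itself, hides the player and shows W_MagicShop.
; A second interact or the player leaving the sphere closes it and restores view and input.
; The construction script applies the chosen mesh and an idle or talking animation per NPC.
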(event OnComponentEndOverlap(Sphere)
  (params (OverlappedComponent :type Primitive%20Component%20Object%20Reference) (OtherActor :type Actor%20Object%20Reference) (OtherComp :type Primitive%20Component%20Object%20Reference) (OtherBodyIndex :type Integer))
  (if (and (Variables|Default|GetIsShopOpen) (Actor|ActorHasTag OtherActor "Player"))
    (CallFunction|CheckifShopNeedstoClose)))

(event Custom|ShowShop
  (bind _returnvalue (Game|GetPlayerController 0))
  (bind _returnvalue_2 (UserInterface|CreateWidget "/Game/ProjectDawn/Blueprints/HUD/MagicShop/W_MagicShop.W_MagicShop_C"))
  (bind _output_get (Variables|Default|SetShopWidgetRef _returnvalue_2))
  (Variables|/Game/ProjectDawn/Blueprints/HUD/MagicShop/W_MagicShop.W_MagicShop_C|SetTeacher _returnvalue_2 self)
  (UserInterface|Viewport|AddtoViewport _returnvalue_2 0)
  (Input|SetInputModeGameandUI _returnvalue _output_get "DoNotLock" true false)
  (Variables|/Script/Engine.PlayerController|SetbShowMouseCursor _returnvalue true)
  (Variables|Default|SetIsShopOpen true))

(event Custom|CheckIfShopNeedsToClose
  (bind _returnvalue (Game|GetPlayerController 0))
  (bind _spellsexpected (Variables|Default|GetSpellsExpected))
  (bind _playerref (Variables|Default|GetPlayerRef))
  (if (Variables|Default|GetIsShopOpen)
    (Widget|RemovefromParent (Variables|Default|GetShopWidgetRef))
    (Input|SetInputModeGameOnly _returnvalue false)
    (Variables|/Script/Engine.PlayerController|SetbShowMouseCursor _returnvalue false)
    (Variables|Default|SetIsShopOpen false)
    (Game|Player|SetViewTargetwithBlend (Game|GetPlayerController 0) (Game|Player|GetPlayerPawn 0) 0.5 "VTBlend_Linear" 0.0 false)
    (Rendering|SetActorHiddenInGame _playerref false)
    (Variables|/Game/ProjectDawn/Blueprints/BP_HeroBase.BP_HeroBase_C|SetIsMagicTeacherScreenOpen _playerref false)
    (else
      (for _index (range 0 (- (Utilities|Array|Length _spellsexpected) 1))
        (bind _returnvalue_2 (Utilities|GetDataTableRow "/Game/ProjectDawn/Blueprints/Magic/Data/DT_Spells.DT_Spells" (Utilities|String|StringToName (Utilities|String|EnumtoString (Utilities|Array|Get(acopy) _spellsexpected _index))))
          (:then
            (Utilities|Array|AddUnique (Variables|Default|GetSpellInventory) _returnvalue_2)
            (Game|Player|SetViewTargetwithBlend (Game|GetPlayerController 0) self 0.5 "VTBlend_Linear" 0.0 false)
            (Rendering|SetActorHiddenInGame (Variables|Default|GetPlayerRef) true))))
      (CallFunction|ShowShop)
      (Variables|/Game/ProjectDawn/Blueprints/BP_HeroBase.BP_HeroBase_C|SetIsMagicTeacherScreenOpen (Variables|Default|GetPlayerRef) true))))

(event Collision|EventActorBeginOverlap
  (params (OtherActor :type Actor%20Object%20Reference)))

(event EventTick
  (params (DeltaSeconds :type Float%20%28single-precision%29)))

(event EventInteract
  (bind _returnvalue (Game|GetPlayerController 0))
  (bind _spellsexpected (Variables|Default|GetSpellsExpected))
  (bind _playerref (Variables|Default|GetPlayerRef))
  (if (Variables|Default|GetIsShopOpen)
    (Widget|RemovefromParent (Variables|Default|GetShopWidgetRef))
    (Input|SetInputModeGameOnly _returnvalue false)
    (Variables|/Script/Engine.PlayerController|SetbShowMouseCursor _returnvalue false)
    (Variables|Default|SetIsShopOpen false)
    (Game|Player|SetViewTargetwithBlend (Game|GetPlayerController 0) (Game|Player|GetPlayerPawn 0) 0.5 "VTBlend_Linear" 0.0 false)
    (Rendering|SetActorHiddenInGame _playerref false)
    (Variables|/Game/ProjectDawn/Blueprints/BP_HeroBase.BP_HeroBase_C|SetIsMagicTeacherScreenOpen _playerref false)
    (else
      (for _index (range 0 (- (Utilities|Array|Length _spellsexpected) 1))
        (bind _returnvalue_2 (Utilities|GetDataTableRow "/Game/ProjectDawn/Blueprints/Magic/Data/DT_Spells.DT_Spells" (Utilities|String|StringToName (Utilities|String|EnumtoString (Utilities|Array|Get(acopy) _spellsexpected _index))))
          (:then
            (Utilities|Array|AddUnique (Variables|Default|GetSpellInventory) _returnvalue_2)
            (Game|Player|SetViewTargetwithBlend (Game|GetPlayerController 0) self 0.5 "VTBlend_Linear" 0.0 false)
            (Rendering|SetActorHiddenInGame (Variables|Default|GetPlayerRef) true))))
      (CallFunction|ShowShop)
      (Variables|/Game/ProjectDawn/Blueprints/BP_HeroBase.BP_HeroBase_C|SetIsMagicTeacherScreenOpen (Variables|Default|GetPlayerRef) true))))

(event EventBeginPlay
  (bind _asbp_hero_base (Utilities|Casting|CastToBP_HeroBase (Game|GetPlayerCharacter 0)))
  (Variables|Default|SetPlayerRef _asbp_hero_base))

(fn ConstructionScript
  (bind _magicteacher (Variables|Default|GetMagicTeacher))
  (|CallParentFunction)
  (Components|SkeletalMesh|SetSkeletalMeshAsset _magicteacher (Variables|Default|GetPickSkeletalMesh))
  (Components|Animation|OverrideAnimationData _magicteacher (Utilities|Select :Index (Variables|Default|GetNPCList) :NewEnumerator0 "/Game/ProjectDawn/Characters/NPC/ShopKeeps/001_Ichigo/Animations/Ichigo_talking.Ichigo_talking" :NewEnumerator1 "/Game/ProjectDawn/Characters/NPC/MagicTeachers/002_Midnight/Animations/MidnightIdle.MidnightIdle" :NewEnumerator5 0 :NewEnumerator6 0 :NewEnumerator7 0 :NewEnumerator8 0 :NewEnumerator9 "/Game/ProjectDawn/Characters/NPC/MagicTeachers/001_Angelica/Anims/AngelicaIdle.AngelicaIdle" :NewEnumerator10 0) true true 0.0 1.0))