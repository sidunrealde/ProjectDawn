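; BP_TargetDrone is a destructible drone prop that serves as a rotating target.
; On BeginPlay it randomly picks clockwise or counterclockwise yaw spin at a fixed speed through its RotatingMovement component.
; Any damage, regardless of amount, spawns a spark destruction emitter at the Drone component's transform and destroys the actor.
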(event EventBeginPlay
  (bind _rotatingmovement (Variables|Default|GetRotatingMovement))
  (if (Math|Random|RandomBool)
    (Variables|/Script/Engine.RotatingMovementComponent|SetRotationRate _rotatingmovement "0.000000,45.000000,0.000000")
    (else
      (Variables|/Script/Engine.RotatingMovementComponent|SetRotationRate _rotatingmovement "0.000000,-45.000000,0.000000"))))

(event Game|Damage|EventAnyDamage
  (params (Damage :type Float%20%28single-precision%29) (DamageType :type Damage%20Type%20Object%20Reference) (InstigatedBy :type Controller%20Object%20Reference) (DamageCauser :type Actor%20Object%20Reference))
  (bind _drone (Variables|Default|GetDrone))
  (bind _returnvalue (Transformation|GetWorldTransform _drone))
  (Effects|SpawnEmitteratLocation "/Game/ProjectDawn/FX/CascadeParticleSystem/Enemy/FX_DroneDestroy_sparks.FX_DroneDestroy_sparks" (.location _returnvalue) (.rotation _returnvalue) (* (.scale _returnvalue) 1.0))
  (Actor|DestroyActor))

(fn ConstructionScript)