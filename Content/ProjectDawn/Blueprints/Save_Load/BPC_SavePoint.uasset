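; Interactable save point that opens and closes the save screen for the player hero.
; Interact toggles the W_SaveScreen widget, cursor and input mode, but only when no other tracked hero menu is open.
; Opening passes itself to the widget and stores the save point location on the hero.
; Leaving the sphere closes an open screen, though only for actors passing a tag check set to None.
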(event OnComponentEndOverlap(Sphere)
  (params (OverlappedComponent :type Primitive%20Component%20Object%20Reference) (OtherActor :type Actor%20Object%20Reference) (OtherComp :type Primitive%20Component%20Object%20Reference) (OtherBodyIndex :type Integer))
  (if (and (Variables|Default|GetIsSaveScreenOpen) (Actor|ActorHasTag OtherActor "None"))
    (CallFunction|CheckifMenuNeedstoClose)))

(event Custom|CheckIfMenuNeedsToClose
  (bind _returnvalue (Game|GetPlayerController 0))
  (bind _returnvalue_2 (Game|GetPlayerController 0))
  (bind _playerref (Variables|Default|GetPlayerRef))
  (if (Variables|Default|GetIsSaveScreenOpen)
    (Widget|RemovefromParent (Variables|Default|GetSaveScreenRef))
    (Variables|/Script/Engine.PlayerController|SetbShowMouseCursor _returnvalue false)
    (Input|SetInputModeGameOnly _returnvalue false)
    (Variables|Default|SetIsSaveScreenOpen false)
    (Variables|/Game/ProjectDawn/Blueprints/BP_HeroBase.BP_HeroBase_C|SetIsSaveScreenOpen (Variables|Default|GetPlayerRef) false)
    (else
      (bind _returnvalue_3 (UserInterface|CreateWidget "/Game/ProjectDawn/Blueprints/HUD/SaveSystem/W_SaveScreen.W_SaveScreen_C"))
      (Variables|/Game/ProjectDawn/Blueprints/HUD/SaveSystem/W_SaveScreen.W_SaveScreen_C|SetSavePoint _returnvalue_3 self)
      (Variables|Default|SetSaveScreenRef _returnvalue_3)
      (UserInterface|Viewport|AddtoViewport _returnvalue_3 0)
      (Variables|/Script/Engine.PlayerController|SetbShowMouseCursor _returnvalue_2 true)
      (Input|SetInputModeGameandUI _returnvalue_2 _returnvalue_3 "DoNotLock" true false)
      (Variables|Default|SetIsSaveScreenOpen true)
      (Variables|/Game/ProjectDawn/Blueprints/BP_HeroBase.BP_HeroBase_C|SetIsSaveScreenOpen _playerref true)
      (Variables|/Game/ProjectDawn/Blueprints/BP_HeroBase.BP_HeroBase_C|SetSavePointLocation _playerref (Variables|Default|GetSPLocation)))))

(event EventBeginPlay
  (bind _asbp_hero_base (Utilities|Casting|CastToBP_HeroBase (Game|GetPlayerCharacter 0)))
  (Variables|Default|SetPlayerRef _asbp_hero_base))

(event EventInteract
  (bind _returnvalue (Game|GetPlayerController 0))
  (bind _returnvalue_2 (Game|GetPlayerController 0))
  (bind _playerref (Variables|Default|GetPlayerRef))
  (bind _playerref_2 (Variables|Default|GetPlayerRef))
  (if (not (Math|Boolean|ORBoolean (Variables|/Game/ProjectDawn/Blueprints/BP_HeroBase.BP_HeroBase_C|GetIsCraftingScreenOpen _playerref) (Variables|/Game/ProjectDawn/Blueprints/BP_HeroBase.BP_HeroBase_C|GetIsEnemyLootScreenOpen _playerref) (Variables|/Game/ProjectDawn/Blueprints/BP_HeroBase.BP_HeroBase_C|GetIsFastTravelScreenOpen _playerref) (Variables|/Game/ProjectDawn/Blueprints/BP_HeroBase.BP_HeroBase_C|GetIsMenuOpen _playerref) (Variables|/Game/ProjectDawn/Blueprints/BP_HeroBase.BP_HeroBase_C|GetIsQuestLogOpen _playerref) (Variables|/Game/ProjectDawn/Blueprints/BP_HeroBase.BP_HeroBase_C|GetIsSpellBookOpen _playerref)))
    (if (Variables|Default|GetIsSaveScreenOpen)
      (Widget|RemovefromParent (Variables|Default|GetSaveScreenRef))
      (Variables|/Script/Engine.PlayerController|SetbShowMouseCursor _returnvalue false)
      (Input|SetInputModeGameOnly _returnvalue false)
      (Variables|Default|SetIsSaveScreenOpen false)
      (Variables|/Game/ProjectDawn/Blueprints/BP_HeroBase.BP_HeroBase_C|SetIsSaveScreenOpen (Variables|Default|GetPlayerRef) false)
      (else
        (bind _returnvalue_3 (UserInterface|CreateWidget "/Game/ProjectDawn/Blueprints/HUD/SaveSystem/W_SaveScreen.W_SaveScreen_C"))
        (Variables|/Game/ProjectDawn/Blueprints/HUD/SaveSystem/W_SaveScreen.W_SaveScreen_C|SetSavePoint _returnvalue_3 self)
        (Variables|Default|SetSaveScreenRef _returnvalue_3)
        (UserInterface|Viewport|AddtoViewport _returnvalue_3 0)
        (Variables|/Script/Engine.PlayerController|SetbShowMouseCursor _returnvalue_2 true)
        (Input|SetInputModeGameandUI _returnvalue_2 _returnvalue_3 "DoNotLock" true false)
        (Variables|Default|SetIsSaveScreenOpen true)
        (Variables|/Game/ProjectDawn/Blueprints/BP_HeroBase.BP_HeroBase_C|SetIsSaveScreenOpen _playerref_2 true)
        (Variables|/Game/ProjectDawn/Blueprints/BP_HeroBase.BP_HeroBase_C|SetSavePointLocation _playerref_2 (Variables|Default|GetSPLocation))))))

(fn ConstructionScript
  (|CallParentFunction))