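; Player save object (SG_PlayerSave) that persists quest log state and per-quest progress.
; SaveQuestLog copies the active and completed quest lists from the quest log component.
; SaveQuestDetails separately stores each quest's stage and objective progress in a map keyed by quest ID.
; LoadQuests recreates active quests through the component, restores their stage and progress from that map, then overwrites both lists with saved values.
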(fn SaveQuestDetails
  (params (Quest :type BP%20Quest%20Actor%20Base%20Object%20Reference))
  (Utilities|Map|Add (Variables|Default|GetQuestProgress) (Variables|/Game/ProjectDawn/Blueprints/Quest/New/BP_QuestActorBase.BP_QuestActorBase_C|GetQuestID Quest) (Utilities|Struct|MakeDS_QuestSaveData (Variables|/Game/ProjectDawn/Blueprints/Quest/New/BP_QuestActorBase.BP_QuestActorBase_C|GetCurrentObjectiveProgress Quest) (Variables|/Game/ProjectDawn/Blueprints/Quest/New/BP_QuestActorBase.BP_QuestActorBase_C|GetCurrentStage Quest))))

(fn LoadQuests
  (params (QuestLogComponent :type BC%20Quest%20Log%20Component%20Object%20Reference))
  (for _array_element (Variables|Default|GetCurrentActiveQuests)
    (bind _questactor (Default|AddNewQuest QuestLogComponent _array_element))
    (Variables|/Game/ProjectDawn/Blueprints/Quest/New/BP_QuestActorBase.BP_QuestActorBase_C|SetCurrentStage _questactor (.CurrentStage (Utilities|Struct|BreakDS_QuestSaveData (.Value (Utilities|Map|Find (Variables|Default|GetQuestProgress) _array_element)))))
    (Variables|/Game/ProjectDawn/Blueprints/Quest/New/BP_QuestActorBase.BP_QuestActorBase_C|SetCurrentObjectiveProgress _questactor (.Progress (Utilities|Struct|BreakDS_QuestSaveData (.Value (Utilities|Map|Find (Variables|Default|GetQuestProgress) _array_element))))))
  (Variables|/Game/ProjectDawn/Blueprints/Quest/New/BC_QuestLogComponent.BC_QuestLogComponent_C|SetCurrentActiveQuest QuestLogComponent (Variables|Default|GetCurrentActiveQuests))
  (Variables|/Game/ProjectDawn/Blueprints/Quest/New/BC_QuestLogComponent.BC_QuestLogComponent_C|SetCompletedQuests QuestLogComponent (Variables|Default|GetCompletedQuests)))

(fn SaveQuestLog
  (params (QuestLogComponent :type BC%20Quest%20Log%20Component%20Object%20Reference))
  (Variables|Default|SetCompletedQuests (Variables|/Game/ProjectDawn/Blueprints/Quest/New/BC_QuestLogComponent.BC_QuestLogComponent_C|GetCompletedQuests QuestLogComponent))
  (Variables|Default|SetCurrentActiveQuests (Variables|/Game/ProjectDawn/Blueprints/Quest/New/BC_QuestLogComponent.BC_QuestLogComponent_C|GetCurrentActiveQuest QuestLogComponent)))